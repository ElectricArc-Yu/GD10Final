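; BP_GlobalMonitor holds game-wide state: a building ID counter and an item-to-count inventory map.
; GetBuildingID increments and returns the counter, while Add and Remove functions apply item maps to the inventory without clamping.
; CheckInventoryState requires stock strictly above each amount, unlike the single-item check, which accepts equality.
; Its key-existence test searches the input list instead of the inventory, and BeginPlay and Tick are unused.
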(fn `AddInventoryNum`
  (params (InAddList :type "Map of /Game/Core/Item/Enum/E_Miscellaneous Enum to Integer"))
  (bind _currentglobalinventory (`self.CurrentGlobalInventory`))
  (bind _keys (`BlueprintMapLibrary.Map_Keys` InAddList))
  (for _array_element _keys
    (bind (_value _returnvalue) (`BlueprintMapLibrary.Map_Find` _currentglobalinventory _array_element))
    (if _returnvalue
      (bind _value_2 (`BlueprintMapLibrary.Map_Find` InAddList _array_element))
      (`BlueprintMapLibrary.Map_Add` _currentglobalinventory _array_element (+ _value_2 _value))
      (else
        (`BlueprintMapLibrary.Map_Add` _currentglobalinventory _array_element _value_2))))
  (return))

(fn `CheckInventoryState`
  (params (InCheckList :type "Map of /Game/Core/Item/Enum/E_Miscellaneous Enum to Integer"))
  (returns (OutResult :type Boolean))
  (bind _keys (`BlueprintMapLibrary.Map_Keys` InCheckList))
  (for _array_element _keys
    (bind (_value _returnvalue) (`BlueprintMapLibrary.Map_Find` InCheckList _array_element))
    (if _returnvalue
      (if (not (> (`BlueprintMapLibrary.Map_Find` (`self.CurrentGlobalInventory`) _array_element) _value))
        (return false))
      (else
        (return false))))
  (return true))

(fn `CheckInventoryStateWithItem`
  (params (InItem :type "/Game/Core/Item/Enum/E_Miscellaneous Enum" :default "NewEnumerator2") (InRequire :type Integer))
  (returns (OutResult :type Boolean))
  (bind (_value _returnvalue) (`BlueprintMapLibrary.Map_Find` (`self.CurrentGlobalInventory`) InItem))
  (if _returnvalue
    (if (<= InRequire _value)
      (return true)
      (else
        (return false)))
    (else
      (return false))))

(fn `GetBuildingID`
  (returns (Result :type Integer))
  (bind _result (`/Engine/EditorBlueprintResources/StandardMacros.IncrementInt` (`self.CurrentGloabalBuildingID`))
    (:`  `
      (bind _output_get (set `self.CurrentGloabalBuildingID` _result))
      (return _output_get))))

(fn `RemoveInventoryNum`
  (params (InRemoveList :type "Map of /Game/Core/Item/Enum/E_Miscellaneous Enum to Integer"))
  (bind _currentglobalinventory (`self.CurrentGlobalInventory`))
  (bind _keys (`BlueprintMapLibrary.Map_Keys` InRemoveList))
  (for _array_element _keys
    (`BlueprintMapLibrary.Map_Add` _currentglobalinventory _array_element (- (`BlueprintMapLibrary.Map_Find` _currentglobalinventory _array_element) (`BlueprintMapLibrary.Map_Find` InRemoveList _array_element))))
  (return))

(fn `UserConstructionScript`)