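; BP_Mark is a hologram marker that shows whether it overlaps an existing BP_Building, apparently as a placement preview.
; Every Tick it queries overlapping BP_Building actors and stores the result in IsOverlapping.
; It then sets every material slot on its Mesh to the error hologram when overlapping, or to the normal hologram otherwise, reapplying them each frame.
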(event `self.ReceiveBeginPlay`
  (`parent.ReceiveBeginPlay`))

(event `self.ReceiveTick`
  (params (DeltaSeconds :type "Float (single-precision)"))
  (bind _returnvalue (`KismetArrayLibrary.Array_LastIndex` (`MeshComponent.GetMaterials` (`self.Mesh`))))
  (bind _output_get (set `self.IsOverlapping` (`KismetArrayLibrary.Array_IsNotEmpty` (`self.GetOverlappingActors` "/Game/Core/Building/Blueprint/BP_Building.BP_Building_C"))))
  (if _output_get
    (for _index (range (+ _returnvalue 1))
      (`PrimitiveComponent.SetMaterial` (`self.Mesh`) _index "/Game/Arts/Shader/Hologram/MI_Hologram_Simple_Error.MI_Hologram_Simple_Error"))
    (else
      (for _index_2 (range (+ _returnvalue 1))
        (`PrimitiveComponent.SetMaterial` (`self.Mesh`) _index_2 "/Game/Arts/Shader/Hologram/MI_Hologram_Simple.MI_Hologram_Simple")))))

(fn `UserConstructionScript`
  (`parent.UserConstructionScript`))