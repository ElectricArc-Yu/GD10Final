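; Player camera pawn for a top-down building game, handling navigation, building selection and placement via Enhanced Input mapping contexts.
; Movement, spin, drag-pan and curve-driven zoom (arm, pitch, speed, FOV) steer the view.
; Overlaps select buildings and tell the game mode, while Tick toggles their property widget.
; BeginBuild spawns a hologram BP_Mark that snaps to the projected mouse position, feeds MPC_Cropout and becomes the target building unless overlapping.
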(event `self.ReceivePossessed`
  (params (NewController :type "Controller Object Reference"))
  (bind _asbp_player_control (cast `/Game/Core/GameMode/BP_PlayerControl` NewController))
  (add `/Game/Core/GameMode/BP_PlayerControl.KeySwitch` _asbp_player_control (`|CreateDelegate` :!event `InputSwitch`)))

(event `self.ReceiveBeginPlay`
  (bind _returnvalue (pcsubsystem `EnhancedInputLocalPlayerSubsystem` (`self.GetPlayerController`)))
  (`|ExecutionSequence`
    (:`then_0`
      (`self.UpdateZoom`)
      (`KismetSystemLibrary.K2_SetTimerDelegate` (`|CreateDelegate` :!event `MoveTracking`) 0.001667 true))
    (:`then_1`
      (`EnhancedInputSubsystemInterface.AddMappingContext` _returnvalue "/Game/Core/GameMode/Input/IMC_BaseInput.IMC_BaseInput" 0 (struct))
      (`EnhancedInputSubsystemInterface.AddMappingContext` _returnvalue "/Game/Core/GameMode/Input/IMC_VillagerMode.IMC_VillagerMode" 0 (struct)))))

(event `BuildingUI`
  (goto _label :!via `Reset`))

(event `EnhancedInput|/Game/Core/GameMode/Input/IA_Villager`
  (params (ActionValue :type Boolean) (ElapsedSeconds :type "Float (double-precision)") (TriggeredSeconds :type "Float (double-precision)") (InputAction :type "InputAction Object Reference" :default "/Game/Core/GameMode/Input/IA_Villager.IA_Villager"))
  (:`Started`
    (`self.SelectedBuilding`
      (:`then`
        (`/Engine/EditorBlueprintResources/StandardMacros.DoOnce` false :!label _label
          (:`Completed`
            (message `/Game/Core/GameMode/BPI_Player.AddUI` (`GameplayStatics.GetGameMode`) "/Game/Core/UI/BuildingProp/CUI_ChangeRecipe.CUI_ChangeRecipe_C")
            (set `self.SelectedBuilding` null))))
      (:`else`
        (`self.PositionCheck`)
        (`EnhancedInputSubsystemInterface.AddMappingContext` (pcsubsystem `EnhancedInputLocalPlayerSubsystem` (`self.GetPlayerController`)) "/Game/Core/GameMode/Input/IMC_DragMove.IMC_DragMove" 0 (struct)))))
  (:`Canceled`
    (`EnhancedInputSubsystemInterface.RemoveMappingContext` (pcsubsystem `EnhancedInputLocalPlayerSubsystem` (`self.GetPlayerController`)) "/Game/Core/GameMode/Input/IMC_DragMove.IMC_DragMove" (make `ModifyContextOptions` true true) :!label _label_2))
  (:`Completed`
    (goto _label_2)))

(event `EnhancedInput|/Game/Core/GameMode/Input/IA_BuildMode_Active`
  (params (ActionValue :type Boolean) (ElapsedSeconds :type "Float (double-precision)") (TriggeredSeconds :type "Float (double-precision)") (InputAction :type "InputAction Object Reference" :default "/Game/Core/GameMode/Input/IA_BuildMode_Active.IA_BuildMode_Active"))
  (:`Started`
    (`KismetSystemLibrary.Delay` 0.2)
    (`self.SpawnBuildTarget`)))

(event `EnhancedInput|/Game/Core/GameMode/Input/IA_BuildMode_Quit`
  (params (ActionValue :type Boolean) (ElapsedSeconds :type "Float (double-precision)") (TriggeredSeconds :type "Float (double-precision)") (InputAction :type "InputAction Object Reference" :default "/Game/Core/GameMode/Input/IA_BuildMode_Quit.IA_BuildMode_Quit"))
  (:`Canceled`
    (`self.DestroySpawn` :!label _label_3)
    (`self.SwitchBuildMode` false)
    (`/Game/Core/GameMode/BP_BaseMode_UI.BackUI` (cast `/Game/Core/GameMode/BP_BaseMode_UI` (`GameplayStatics.GetGameMode`) :!pure true)))
  (:`Completed`
    (goto _label_3)))

(event `EnhancedInput|/Game/Core/GameMode/Input/IA_Move`
  (params (ActionValue :type "Vector2D Structure") (ElapsedSeconds :type "Float (double-precision)") (TriggeredSeconds :type "Float (double-precision)") (InputAction :type "InputAction Object Reference" :default "/Game/Core/GameMode/Input/IA_Move.IA_Move"))
  ;[1 1 1] Movement
  (:`Triggered`
    (`self.AddMovementInput` (`self.GetActorForwardVector`) ActionValue_Y)
    (`self.AddMovementInput` (`self.GetActorRightVector`) ActionValue_X)))

(event `self.BeginBuild`
  (params (TargetClass :type "/Game/Core/GameMode/Interactable/BP_Interactable Class Reference") (Model :type "StaticMesh Object Reference"))
  ;[1 1 1] ？？？？
  (set `self.TargetSpawnClass` TargetClass)
  (`/Engine/EditorBlueprintResources/StandardMacros.IsValid` (`self.Spawn`)
    (:`Is Valid`
      (`self.K2_DestroyActor` (`self.Spawn`)))
    (:`Is Not Valid`
      _))
  (bind _returnvalue (`|SpawnActorFromClass` "/Game/Core/GameMode/Interactable/BP_Mark.BP_Mark_C" (`KismetMathLibrary.Conv_VectorToTransform` (`self.K2_GetActorLocation`)) "Undefined" "OverrideRootScale" null null))
  (bind _output_get (set `self.Spawn` _returnvalue))
  (`StaticMeshComponent.SetStaticMesh` (`/Game/Core/GameMode/Interactable/BP_Interactable.Mesh` _output_get) Model)
  (for _index (range (+ (`KismetArrayLibrary.Array_LastIndex` (`MeshComponent.GetMaterials` (`/Game/Core/GameMode/Interactable/BP_Interactable.Mesh` _output_get))) 1))
    (`PrimitiveComponent.SetMaterial` (`/Game/Core/GameMode/Interactable/BP_Interactable.Mesh` _returnvalue) _index "/Game/Arts/Shader/Hologram/MI_Hologram_Simple.MI_Hologram_Simple"))
  (`/Game/Core/GameMode/Interactable/BP_Interactable.Placement` _output_get)
  (bind _returnvalue_2 (`|GetDataTableRow` "/Game/Core/Building/Data/DT_Building.DT_Building" (`KismetStringLibrary.Conv_StringToName` (`.RightS` (`KismetStringLibrary.Split` (`KismetSystemLibrary.GetObjectName` Model) "_"))))
    (:`then`
      (bind _box (`/Game/Core/GameMode/Interactable/BP_Interactable.Box` _output_get))
      (bind (_x _y) (`KismetMathLibrary.BreakVector2D` (`.Area_12_8ED1BBBA4648017C62688BB441E48DE3` (break `/Game/Core/Building/Struct/Building/ST_Building` _returnvalue_2))))
      (bind _returnvalue_3 (* _x 100.0))
      (bind _returnvalue_4 (* _y 100.0))
      (`BoxComponent.SetBoxExtent` _box (`KismetMathLibrary.MakeVector_NetQuantize` (- _returnvalue_3 2.0) (- _returnvalue_4 2.0) 64.0) true)
      (`SceneComponent.K2_AddLocalOffset` _box (`KismetMathLibrary.MakeVector` _returnvalue_3 _returnvalue_4) false true))))

(event `EnhancedInput|/Game/Core/GameMode/Input/IA_Zoom`
  (params (ActionValue :type "Float (double-precision)") (ElapsedSeconds :type "Float (double-precision)") (TriggeredSeconds :type "Float (double-precision)") (InputAction :type "InputAction Object Reference" :default "/Game/Core/GameMode/Input/IA_Zoom.IA_Zoom"))
  ;[1 1 1] Movement
  (:`Triggered`
    (set `self.ZoomDirection` ActionValue)
    (`self.UpdateZoom`)
    (`self.Dof`)))

(event `EnhancedInput|/Game/Core/GameMode/Input/IA_DragMove`
  (params (ActionValue :type "Float (double-precision)") (ElapsedSeconds :type "Float (double-precision)") (TriggeredSeconds :type "Float (double-precision)") (InputAction :type "InputAction Object Reference" :default "/Game/Core/GameMode/Input/IA_DragMove.IA_DragMove"))
  ;[1 1 1] Movement
  (:`Triggered`
    (`self.TrackMove`)))

(event `EnhancedInput|/Game/Core/GameMode/Input/IA_Spin`
  (params (ActionValue :type "Float (double-precision)") (ElapsedSeconds :type "Float (double-precision)") (TriggeredSeconds :type "Float (double-precision)") (InputAction :type "InputAction Object Reference" :default "/Game/Core/GameMode/Input/IA_Spin.IA_Spin"))
  ;[1 1 1] Movement
  (:`Triggered`
    (`self.K2_AddActorLocalRotation` (`KismetMathLibrary.MakeRotator` 0.0 0.0 ActionValue))))

(event `self.ReceiveTick`
  (params (DeltaSeconds :type "Float (single-precision)"))
  (`|ExecutionSequence`
    (:`then_0`
      (`self.Spawn`
        (:`then`
          (`self.UpdateBuildAsset`))
        (:`else`)))
    (:`then_1`
      ;[1 1 1] BuildingProp
      (`self.SelectedBuilding`
        (:`then`
          (`self.BuildingProp`
            (:`then`
              (`Widget.SetVisibility` (`self.BuildingProp`) "Visible"))
            (:`else`
              (bind _returnvalue (`|CreateWidget` "/Game/Core/UI/BuildingProp/CUI_BuildingProp.CUI_BuildingProp_C"))
              (`UserWidget.AddToViewport` _returnvalue 0)
              (set `self.BuildingProp` _returnvalue))))
        (:`else`
          (`self.BuildingProp`
            (:`then`
              (`Widget.SetVisibility` (`self.BuildingProp`) "Hidden"))
            (:`else`)))))))

(event `self.ReceiveActorBeginOverlap`
  (params (OtherActor :type "Actor Object Reference"))
  (if (not (`self.IsSelected`))
    (`self.SelectedBuilding`
      (:`then`)
      (:`else`
        (bind _asbp_building (cast `/Game/Core/Building/Blueprint/BP_Building` OtherActor))
        (bind _output_get (set `self.SelectedBuilding` _asbp_building))
        (message `/Game/Core/GameMode/BPI_Player.SelectBuilding` (`GameplayStatics.GetGameMode`) _output_get)
        (set `self.IsSelected` false)))))

(event `self.ReceiveActorEndOverlap`
  (params (OtherActor :type "Actor Object Reference"))
  (set `self.SelectedBuilding` null :!label _label_4)
  (set `self.IsSelected` false))

(event `self.Box.OnComponentEndOverlap`
  (params (OverlappedComponent :type "PrimitiveComponent Object Reference") (OtherActor :type "Actor Object Reference") (OtherComp :type "PrimitiveComponent Object Reference") (OtherBodyIndex :type Integer))
  (cast `/Game/Core/Building/Blueprint/BP_Building` OtherActor)
  (goto _label_4))

(fn `CornersInNav`
  (returns (NewParam :type Boolean))
  (bind _array (`|MakeArray` null :!type "Actor Object Reference"))
  (bind (_origin _boxextent) (`KismetSystemLibrary.GetComponentBounds` (`/Game/Core/GameMode/Interactable/BP_Interactable.Box` (`self.Spawn`))))
  (bind _returnvalue (* (.y _boxextent) 1.05))
  (bind _returnvalue_2 (* (.x _boxextent) 1.05))
  (bind _returnvalue_3 (* _returnvalue -1.0))
  (bind _returnvalue_4 (* _returnvalue_2 -1.0))
  (bind _x (.x (+ _origin (`KismetMathLibrary.MakeVector` _returnvalue_2 _returnvalue))))
  (bind _y (.y (+ _origin (`KismetMathLibrary.MakeVector` _returnvalue_2 _returnvalue))))
  (bind _x_2 (.x (+ _origin (`KismetMathLibrary.MakeVector` _returnvalue_4 _returnvalue_3))))
  (bind _y_2 (.y (+ _origin (`KismetMathLibrary.MakeVector` _returnvalue_4 _returnvalue_3))))
  (bind _x_3 (.x (+ _origin (`KismetMathLibrary.MakeVector` _returnvalue_4 _returnvalue))))
  (bind _y_3 (.y (+ _origin (`KismetMathLibrary.MakeVector` _returnvalue_4 _returnvalue))))
  (bind _x_4 (.x (+ _origin (`KismetMathLibrary.MakeVector` _returnvalue _returnvalue_3))))
  (bind _y_4 (.y (+ _origin (`KismetMathLibrary.MakeVector` _returnvalue _returnvalue_3))))
  (bind (_outhits _returnvalue_5) (`KismetSystemLibrary.LineTraceMulti` (`KismetMathLibrary.MakeVector` _x _y 100.0) (`KismetMathLibrary.MakeVector` _x _y -1.0) "TraceTypeQuery1" false _array))
  (if _returnvalue_5
    (bind (_outhits_2 _returnvalue_6) (`KismetSystemLibrary.LineTraceMulti` (`KismetMathLibrary.MakeVector` _x_3 _y_3 100.0) (`KismetMathLibrary.MakeVector` _x_3 _y_3 -1.0) "TraceTypeQuery1" false _array))
    (if _returnvalue_6
      (bind (_outhits_3 _returnvalue_7) (`KismetSystemLibrary.LineTraceMulti` (`KismetMathLibrary.MakeVector` _x_4 _y_4 100.0) (`KismetMathLibrary.MakeVector` _x_4 _y_4 -1.0) "TraceTypeQuery1" false _array))
      (if _returnvalue_7
        (bind (_outhits_4 _returnvalue_8) (`KismetSystemLibrary.LineTraceMulti` (`KismetMathLibrary.MakeVector` _x_2 _y_2 100.0) (`KismetMathLibrary.MakeVector` _x_2 _y_2 -1.0) "TraceTypeQuery1" false _array))
        (if _returnvalue_8
          (set `self.OnIsland` true)
          (else
            (set `self.OnIsland` false :!label _label)))
        (else
          (goto _label)))
      (else
        (goto _label)))
    (else
      (goto _label)))
  (return (`self.OnIsland`)))

(fn `CreateBuildOverlay`
  (`self.SpawnOverlay`
    (:`then`)
    (:`else`
      (bind _returnvalue (`AddComponent|NODE_AddStaticMeshComponent-0` :`RelativeTransform` (`KismetMathLibrary.MakeTransform` (0.0 0.0 0.0) (struct) (/ (`.BoxExtent` (`self.GetActorBounds` (`self.Spawn`) false false)) 50.0))))
      (bind _output_get (set `self.SpawnOverlay` _returnvalue))
      (`SceneComponent.K2_AttachToComponent` _output_get (`/Game/Core/GameMode/Interactable/BP_Interactable.Mesh` (`self.Spawn`)) "None" "SnapToTarget" "KeepWorld" "KeepWorld" true))))

(fn `DestroySpawn`
  (`self.K2_DestroyActor` (`self.Spawn`)))

(fn `Dof`
  (set `CameraComponent.PostProcessSettings` (make `PostProcessSettings` :`DepthOfFieldFocalDistance` (`SpringArmComponent.TargetArmLength` (`self.SpringArm`))) (`self.Camera`)))

(fn `GetPlayerController`
  (returns (GenericPC :type "PlayerController Object Reference"))
  (return (cast `PlayerController` (`self.GetController`) :!pure true)))

(fn `InputSwitch`
  (params (NewInput :type "/Game/Core/GameMode/Input/E_InputType Enum" :default "NewEnumerator0"))
  (bind _output_get (set `self.Input Type` NewInput))
  (switch `/Game/Core/GameMode/Input/E_InputType` _output_get))

(fn `MoveTracking`
  (bind (_direction _srtength) (`self.EdgeMove`))
  (`self.UpdateCursorPosition`)
  (`self.AddMovementInput` _direction _srtength)
  (`SceneComponent.K2_SetWorldLocation` (`self.Box`) (+ (`self.ProjectMouse`) (0.0 0.0 10.0)) false false))

(fn `PositionCheck`
  (set `self.Target Handle` (`self.ProjectMouse`)))

(fn `RemoveResources`)

(fn `SpawnBuildTarget`
  (bind _spawn (`self.Spawn`))
  (if (not (`/Game/Core/GameMode/Interactable/BP_Mark.IsOverlapping` (cast `/Game/Core/GameMode/Interactable/BP_Mark` _spawn :!pure true)))
    (`|SpawnActorFromClass` (`self.TargetSpawnClass`) (`self.GetTransform` _spawn) "Undefined" "MultiplyWithRoot" null null)
    (`self.RemoveResources`)
    (`self.UpdateBuildAsset`)))

(fn `SwitchBuildMode`
  (params (IsSwitchToBuildMode :type Boolean))
  (bind _returnvalue (pcsubsystem `EnhancedInputLocalPlayerSubsystem` (`self.GetPlayerController`)))
  (if IsSwitchToBuildMode
    (`EnhancedInputSubsystemInterface.RemoveMappingContext` _returnvalue "/Game/Core/GameMode/Input/IMC_VillagerMode.IMC_VillagerMode" (struct))
    (`EnhancedInputSubsystemInterface.AddMappingContext` _returnvalue "/Game/Core/GameMode/Input/IMC_BuildMode.IMC_BuildMode" 0 (struct))
    (else
      (`EnhancedInputSubsystemInterface.RemoveMappingContext` _returnvalue "/Game/Core/GameMode/Input/IMC_BuildMode.IMC_BuildMode" (struct))
      (`EnhancedInputSubsystemInterface.AddMappingContext` _returnvalue "/Game/Core/GameMode/Input/IMC_VillagerMode.IMC_VillagerMode" 0 (struct))))
  (return))

(fn `TrackMove`
  (bind (_intersection _screenpos _returnvalue) (`self.ProjectMouse`))
  (bind _springarm (`self.SpringArm`))
  (bind (_socketoffset_x _socketoffset_y _socketoffset_z) (`KismetMathLibrary.BreakVector` (`SpringArmComponent.SocketOffset` _springarm)))
  (if _returnvalue
    (bind _output_get (set `self.StoredMove` (- (`self.Target Handle`) _intersection (- (+ (* (`SceneComponent.GetForwardVector` _springarm) (- (`SpringArmComponent.TargetArmLength` _springarm) _socketoffset_x) -1.0) (* (`SceneComponent.GetUpVector` _springarm) _socketoffset_z) (`SceneComponent.K2_GetComponentLocation` _springarm)) (`SceneComponent.K2_GetComponentLocation` (`self.Camera`))))))
    (`self.K2_AddActorWorldOffset` (`KismetMathLibrary.MakeVector` (.x _output_get) (.y _output_get)))))

(fn `UpdateBuildAsset`
  (bind (_intersection _screenpos _returnvalue) (`self.ProjectMouse`))
  (bind _newparam (`/Game/Core/GameMode/BPF_Shared.Convert to Stepped Pos` _intersection))
  (if _returnvalue
    (bind _spawn (`self.Spawn`)
      (:`then`
        (`self.K2_SetActorLocation` _spawn _newparam false false)
        (if (== (`KismetArrayLibrary.Array_Length` (`self.GetOverlappingActors` (`self.Spawn`) "/Game/Core/GameMode/Interactable/BP_Interactable.BP_Interactable_C")) 0)
          _
          (else
            _))
        (set `self.CanDrop` true)
        (`KismetMaterialLibrary.SetVectorParameterValue` "/Game/Core/GameMode/MPC_Cropout.MPC_Cropout" "Target Position" (make `LinearColor` (.x _newparam) (.y _newparam) (.z _newparam) (`KismetMathLibrary.Conv_BoolToDouble` (`self.CanDrop`)))))
      (:`else`))))

(fn `UpdateCursorPosition`
  (locals (Target :type "Transform Structure"))
  (bind (_returnvalue_location _returnvalue_rotation) (`KismetMathLibrary.BreakTransform` (`SceneComponent.K2_GetComponentToWorld` (`self.Box`))))
  (bind (_origin _boxextent) (`self.GetActorBounds` (`self.SelectedBuilding`) true false))
  (bind _returnvalue (+ (/ (`KismetMathLibrary.GetAbsMax2D` (`KismetMathLibrary.MakeVector2D` (.x _boxextent) (.y _boxextent))) 50.0) (* (`KismetMathLibrary.Sin` (* (`KismetSystemLibrary.GetGameTimeInSeconds`) 5.0)) 0.25) 1.0))
  (switch `/Game/Core/GameMode/Input/E_InputType` (`self.Input Type`)
    (:`NewEnumerator1`
      _)
    (:`NewEnumerator2`
      _))
  (`self.SelectedBuilding`
    (:`then`
      (set `local.Target` (`KismetMathLibrary.MakeTransform` (`KismetMathLibrary.MakeVector` (.x _origin) (.y _origin) 20.0) (struct) (`KismetMathLibrary.MakeVector` _returnvalue _returnvalue 1.0))))
    (:`else`
      (set `local.Target` (`KismetMathLibrary.MakeTransform` _returnvalue_location _returnvalue_rotation (2.0 2.0 1.0)))))
  (`SceneComponent.K2_SetWorldTransform` (`self.Cursor`) (`local.Target`) false false))

(fn `UpdateZoom`
  (bind _springarm (`self.SpringArm`))
  (bind _returnvalue (`CurveFloat.GetFloatValue` (`self.ZoomCurve`) (`self.ZoomValue`)))
  (set `self.ZoomValue` (`KismetMathLibrary.FClamp` (+ (* (`self.ZoomDirection`) 0.01) (`self.ZoomValue`))))
  (set `SpringArmComponent.TargetArmLength` (`KismetMathLibrary.Lerp` 5000.0 80000.0 _returnvalue) _springarm)
  (`SceneComponent.K2_SetRelativeRotation` _springarm (`KismetMathLibrary.MakeRotator` 0.0 (`KismetMathLibrary.Lerp` -40.0 -55.0 _returnvalue)) false false)
  (set `FloatingPawnMovement.MaxSpeed` (`KismetMathLibrary.Lerp` 1000.0 6000.0 _returnvalue) (`self.FloatingPawnMovement`))
  (`self.Dof`)
  (`CameraComponent.SetFieldOfView` (`self.Camera`) (`KismetMathLibrary.Lerp` 20.0 10.0 _returnvalue)))

(fn `UserConstructionScript`)