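; Player controller that tracks whether the player is using gamepad or keyboard and mouse and announces changes.
; A gamepad key press or non-zero mouse movement sets InputType and calls the KeySwitch dispatcher only when the device differs.
; ScanNet multi-line-traces the Visibility channel under the cursor.
; The logic that selects its hits and the switch to Touch are both unwired and never run.
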(event `InputAction|KeyDetect`
  (params (Key :type "Key Structure"))
  ;[1 1 1] Comment
  (:`Pressed`
    (if (`KismetInputLibrary.Key_IsGamepadKey` Key)
      (switch `/Game/Core/GameMode/Input/E_InputType` (`self.InputType`)
        (:`NewEnumerator0`
          _)
        (:`NewEnumerator1`
          _)
        (:`NewEnumerator3`
          _))
      (set `self.InputType` "NewEnumerator2")
      (`self.KeySwitch` (`self.InputType`) :!label _label))))

(event `InputAxis|MouseMove`
  (params (AxisValue :type "Float (single-precision)"))
  ;[1 1 1] Comment
  (if (!= AxisValue 0.0)
    (switch `/Game/Core/GameMode/Input/E_InputType` (`self.InputType`)
      (:`NewEnumerator0`
        _)
      (:`NewEnumerator2`
        _)
      (:`NewEnumerator3`
        _))
    (set `self.InputType` "NewEnumerator1")
    (goto _label)))

(event `self.ReceiveTick`
  (params (DeltaSeconds :type "Float (single-precision)"))
  ;[1 1 1] Comment
)

(fn `ScanNet`
  (returns (isTarget :type Boolean) (OutHits :type "Array of HitResult Structure"))
  (bind (_worldlocation _worlddirection) (`self.DeprojectMousePositionToWorld`))
  (bind (_outhits _returnvalue) (`KismetSystemLibrary.LineTraceMulti` _worldlocation (+ _worldlocation (* _worlddirection 10000.0)) "TraceTypeQuery1"))
  (return _returnvalue _outhits))

(fn `UserConstructionScript`)