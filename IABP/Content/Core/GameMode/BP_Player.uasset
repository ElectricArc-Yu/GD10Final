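; BP_Player is the player's camera pawn, with Enhanced Input move, spin, zoom and drag-pan.
; A curve-shaped zoom value drives spring arm length and pitch, movement speed and FOV, with depth of field following arm length.
; Drag-pan offsets the pawn using cursor, touch or screen-centre projection onto the Z=0 plane, chosen by input type.
; MoveTracking applies edge-scroll movement from that screen point's distance past viewport margins.
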(event `self.ReceivePossessed`
  (params (NewController :type "Controller Object Reference"))
  (bind _asbp_player_control (cast `/Game/Core/GameMode/BP_PlayerControl` NewController))
  (add `/Game/Core/GameMode/BP_PlayerControl.KeySwitch` _asbp_player_control (`|CreateDelegate` :!event `InputSwitch`)))

(event `self.ReceiveBeginPlay`
  (bind _returnvalue (pcsubsystem `EnhancedInputLocalPlayerSubsystem` (`self.GetPlayerController`)))
  (`|ExecutionSequence`
    (:`then_0`
      (`self.UpdateZoom`)
      (`KismetSystemLibrary.K2_SetTimerDelegate` (`|CreateDelegate` :!event `MoveTracking`) 0.001667 true))
    (:`then_1`
      (`EnhancedInputSubsystemInterface.AddMappingContext` _returnvalue "/Game/Core/GameMode/Input/IMC_BaseInput.IMC_BaseInput" 0 (struct))
      (`EnhancedInputSubsystemInterface.AddMappingContext` _returnvalue "/Game/Core/GameMode/Input/IMC_VillagerMode.IMC_VillagerMode" 0 (struct)))))

(event `EnhancedInput|/Game/Core/GameMode/Input/IA_Villager`
  (params (ActionValue :type Boolean) (ElapsedSeconds :type "Float (double-precision)") (TriggeredSeconds :type "Float (double-precision)") (InputAction :type "InputAction Object Reference" :default "/Game/Core/GameMode/Input/IA_Villager.IA_Villager"))
  (:`Started`
    (`self.PositionCheck`)
    (`EnhancedInputSubsystemInterface.AddMappingContext` (pcsubsystem `EnhancedInputLocalPlayerSubsystem` (`self.GetPlayerController`)) "/Game/Core/GameMode/Input/IMC_DragMove.IMC_DragMove" 0 (struct)))
  (:`Canceled`
    (`EnhancedInputSubsystemInterface.AddMappingContext` (pcsubsystem `EnhancedInputLocalPlayerSubsystem` (`self.GetPlayerController`)) "/Game/Core/GameMode/Input/IMC_DragMove.IMC_DragMove" 0 (make `ModifyContextOptions` true true) :!label _label))
  (:`Completed`
    (goto _label)))

(event `EnhancedInput|/Game/Core/GameMode/Input/IA_Move`
  (params (ActionValue :type "Vector2D Structure") (ElapsedSeconds :type "Float (double-precision)") (TriggeredSeconds :type "Float (double-precision)") (InputAction :type "InputAction Object Reference" :default "/Game/Core/GameMode/Input/IA_Move.IA_Move"))
  ;[1 1 1] Movement
  (:`Triggered`
    (`self.AddMovementInput` (`self.GetActorForwardVector`) ActionValue_Y)
    (`self.AddMovementInput` (`self.GetActorRightVector`) ActionValue_X)))

(event `EnhancedInput|/Game/Core/GameMode/Input/IA_Zoom`
  (params (ActionValue :type "Float (double-precision)") (ElapsedSeconds :type "Float (double-precision)") (TriggeredSeconds :type "Float (double-precision)") (InputAction :type "InputAction Object Reference" :default "/Game/Core/GameMode/Input/IA_Zoom.IA_Zoom"))
  ;[1 1 1] Movement
  (:`Triggered`
    (set `self.ZoomDirection` ActionValue)
    (`self.UpdateZoom`)
    (`self.Dof`)))

(event `EnhancedInput|/Game/Core/GameMode/Input/IA_DragMove`
  (params (ActionValue :type "Float (double-precision)") (ElapsedSeconds :type "Float (double-precision)") (TriggeredSeconds :type "Float (double-precision)") (InputAction :type "InputAction Object Reference" :default "/Game/Core/GameMode/Input/IA_DragMove.IA_DragMove"))
  ;[1 1 1] Movement
  (:`Triggered`
    (`self.TrackMove`)))

(event `EnhancedInput|/Game/Core/GameMode/Input/IA_Spin`
  (params (ActionValue :type "Float (double-precision)") (ElapsedSeconds :type "Float (double-precision)") (TriggeredSeconds :type "Float (double-precision)") (InputAction :type "InputAction Object Reference" :default "/Game/Core/GameMode/Input/IA_Spin.IA_Spin"))
  ;[1 1 1] Movement
  (:`Triggered`
    (`self.K2_AddActorLocalRotation` (`KismetMathLibrary.MakeRotator` 0.0 0.0 ActionValue))))

(fn `Dof`
  (set `CameraComponent.PostProcessSettings` (make `PostProcessSettings` :`DepthOfFieldFocalDistance` (`SpringArmComponent.TargetArmLength` (`self.SpringArm`))) (`self.Camera`)))

(fn `GetPlayerController`
  (returns (GenericPC :type "PlayerController Object Reference"))
  (return (cast `PlayerController` (`self.GetController`) :!pure true)))

(fn `InputSwitch`
  (params (NewInput :type "/Game/Core/GameMode/Input/E_InputType Enum" :default "NewEnumerator0"))
  (bind _output_get (set `self.Input Type` NewInput))
  (switch `/Game/Core/GameMode/Input/E_InputType` _output_get))

(fn `MoveTracking`
  (bind (_direction _srtength) (`self.EdgeMove`))
  (`self.AddMovementInput` _direction _srtength))

(fn `PositionCheck`
  (set `self.Target Handle` (`self.ProjectMouse`)))

(fn `TrackMove`
  (bind (_intersection _screenpos _returnvalue) (`self.ProjectMouse`))
  (if _returnvalue
    (bind _output_get (set `self.StoredMove` (- (`self.Target Handle`) _intersection)))
    (`self.K2_AddActorWorldOffset` (`KismetMathLibrary.MakeVector` (.x _output_get) (.y _output_get)))))

(fn `UpdateZoom`
  (bind _springarm (`self.SpringArm`))
  (bind _returnvalue (`CurveFloat.GetFloatValue` (`self.ZoomCurve`) (`self.ZoomValue`)))
  (set `self.ZoomValue` (`KismetMathLibrary.FClamp` (+ (* (`self.ZoomDirection`) 0.01) (`self.ZoomValue`))))
  (set `SpringArmComponent.TargetArmLength` (`KismetMathLibrary.Lerp` 800.0 40000.0 _returnvalue) _springarm)
  (`SceneComponent.K2_SetRelativeRotation` _springarm (`KismetMathLibrary.MakeRotator` 0.0 (`KismetMathLibrary.Lerp` -40.0 -55.0 _returnvalue)) false false)
  (set `FloatingPawnMovement.MaxSpeed` (`KismetMathLibrary.Lerp` 1000.0 6000.0 _returnvalue) (`self.FloatingPawnMovement`))
  (`self.Dof`)
  (`CameraComponent.SetFieldOfView` (`self.Camera`) (`KismetMathLibrary.Lerp` 20.0 10.0 _returnvalue)))

(fn `UserConstructionScript`)