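; Base game mode Blueprint that sets up the game's UI layer and holds building list and resource data.
; BeginPlay creates UI_Layer_Game, adds it to the viewport and activates it, and AddUI pushes items onto its widget stack.
; BuildingList stores the building list, and CheckReesource looks up an entry in the Resource map.
; GetCurrentResource and RemoveResource are stubs returning default values.
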(event `self.ReceiveBeginPlay`
  (bind _returnvalue (`|CreateWidget` "/Game/Core/UI/common/UI_Layer_Game.UI_Layer_Game_C"))
  (`UserWidget.AddToViewport` _returnvalue 0)
  (bind _output_get (set `self.UI HUD Test` _returnvalue))
  (`CommonActivatableWidget.ActivateWidget` _output_get))

(event `self.BuildingList`
  (params (NewParam :type "/Game/Core/GameMode/Interactable/Extras/E_BuidingList Enum" :default "NewEnumerator0"))
  (set `self.List_Building` NewParam))

(event `/Game/Core/GameMode/BPI_Player.AddUI`
  (params (NewParam :type "CommonActivatableWidget Class Reference"))
  (`/Game/Core/UI/common/UI_Layer_Game.Add Stack Item` (`self.UI HUD Test`) NewParam))

(fn `CheckReesource`
  (params (NewParam :type "/Game/Core/GameMode/Interactable/Extras/E_ResourceType Enum" :default "NewEnumerator0"))
  (returns (NewParam1 :type Boolean) (NewParam2 :type Integer))
  (bind (_value _returnvalue) (`BlueprintMapLibrary.Map_Find` (`self.Resource`) NewParam))
  (return _returnvalue _value))

(fn `GetCurrentResource`
  (returns (Resource :type "/Game/Core/GameMode/Interactable/Extras/E_ResourceType Enum"))
  (return "NewEnumerator0"))

(fn `RemoveResource`
  (returns (TargetResource :type "/Game/Core/GameMode/Interactable/Extras/E_ResourceType Enum") (Value :type Integer))
  (return "NewEnumerator0" 0))

(fn `UserConstructionScript`)