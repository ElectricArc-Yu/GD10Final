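; Base dock building that joins a pipeline to an adjacent building, with output docks distinguished by a cast to BP_Building_OutputDock.
; Every tick it line-traces each contact direction and picks a dock mesh from the pipe and building sides found.
; It then stores the contacted building and links itself as the pipeline's precursor for output docks, or successor otherwise.
; Item selection and transfer functions are stubs with unreachable leftover logic.
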(event `self.Event Refresh Static Mesh`
  (`BlueprintMapLibrary.Map_Clear` (`self.PipelineContactInfo`))
  (bind _enumvalue (foreach `/Game/Core/Building/Enum/E_ContactInfo` true)
    (:`LoopBody`
      (`self.CastRayToCheckContact` _enumvalue))
    (:`then`
      (bind _outdockstaticmeshinfo (`self.GetCorrectDockStaticMeshInfo` (`self.PipelineContactInfo`)))
      (set `self.CurrentStaticMeshType` (`|EnumInequality` _outdockstaticmeshinfo "NewEnumerator0"))
      (`self.ChangeStaticMeshByEnum` "NewEnumerator11" _outdockstaticmeshinfo)
      (`self.RefreshPSNode`))))

(event `self.ReceiveTick`
  (params (DeltaSeconds :type "Float (single-precision)"))
  (`self.Event Refresh Static Mesh`)
  (bind _outresult (`self.TickTimer` DeltaSeconds))
  (if _outresult
    _))

(fn `CastRayToCheckContact`
  (params (InDerection :type "/Game/Core/Building/Enum/E_ContactInfo Enum" :default "NewEnumerator0"))
  (locals (TempOrigin :type "Vector Structure") (TempDerection :type "Vector Structure"))
  (bind _returnvalue (`SceneComponent.K2_GetComponentLocation` (`self.MainBuilding`)))
  (bind (_origin _derection) (break `/Game/Core/Building/Struct/TransportNetwork/ST_RayInfo` (`BlueprintMapLibrary.Map_Find` (`self.RaycastMap`) InDerection)))
  (set `local.TempOrigin` _origin)
  (set `local.TempDerection` _derection)
  (bind (_outhit _returnvalue_2) (`KismetSystemLibrary.LineTraceSingle` :`Start` (+ _returnvalue (`local.TempOrigin`)) :`End` (+ _returnvalue (`local.TempDerection`)) :`TraceChannel` "TraceTypeQuery1" :`DrawDebugType` (`self.Draw Debug Type`)))
  (if _returnvalue_2
    (bind (_bblockinghit _binitialoverlap _time _distance _location _impactpoint _normal _impactnormal _physmat _hitactor) (`GameplayStatics.BreakHitResult` _outhit))
    (bind _asbp_building (cast `/Game/Core/Building/Blueprint/BP_Building` _hitactor)
      (:`then`
        (bind _asbp_building_pipeline (cast `/Game/Core/Building/Blueprint/BP_Building_Pipeline` _hitactor)
          (:`then`
            (`BlueprintMapLibrary.Map_Add` (`self.PipelineContactInfo`) (`local.InDerection`) (make `/Game/Core/Building/Struct/TransportNetwork/ST_PipelineContactInfo` true _asbp_building_pipeline null))
            (return))
          (:`CastFailed`
            (`BlueprintMapLibrary.Map_Add` (`self.PipelineContactInfo`) (`local.InDerection`) (make `/Game/Core/Building/Struct/TransportNetwork/ST_PipelineContactInfo` false null _asbp_building))
            (return))))
      (:`CastFailed`
        (return)))
    (else
      (return))))

(fn `GetCorrectDockStaticMeshInfo`
  (params (InPipelineContactInfo :type "Map of /Game/Core/Building/Enum/E_ContactInfo Enum to /Game/Core/Building/Struct/TransportNetwork/ST_PipelineContactInfo Structure"))
  (returns (OutDockStaticMeshInfo :type "/Game/Core/Building/Enum/E_Dock_StaticMeshInfo Enum"))
  (locals (TempBuildingEnum :type "/Game/Core/Building/Enum/E_ContactInfo Enum") (TempPipeEnum :type "/Game/Core/Building/Enum/E_ContactInfo Enum"))
  (if (!= (`BlueprintMapLibrary.Map_Length` InPipelineContactInfo) 2)
    (if (!= (`BlueprintMapLibrary.Map_Length` InPipelineContactInfo) 1)
      (if (> (`BlueprintMapLibrary.Map_Length` InPipelineContactInfo) 2)
        (return "NewEnumerator0")
        (else
          (return "NewEnumerator0")))
      (else
        (bind _keys (`BlueprintMapLibrary.Map_Keys` InPipelineContactInfo))
        (bind _output (`|GetArrayItem` _keys))
        (if (`.PipelineOrBuilding_9_98AA73B24E067DE2AB1C8F83D686ED4F` (break `/Game/Core/Building/Struct/TransportNetwork/ST_PipelineContactInfo` (`BlueprintMapLibrary.Map_Find` InPipelineContactInfo _output)))
          (return (select `/Game/Core/Building/Enum/E_ContactInfo` _output :`NewEnumerator0` "NewEnumerator7" :`NewEnumerator1` "NewEnumerator1" :`NewEnumerator2` "NewEnumerator4" :`NewEnumerator3` "NewEnumerator10" :!type "/Game/Core/Building/Enum/E_Dock_StaticMeshInfo Enum"))
          (else
            (return (select `/Game/Core/Building/Enum/E_ContactInfo` _output :`NewEnumerator0` "NewEnumerator1" :`NewEnumerator1` "NewEnumerator7" :`NewEnumerator2` "NewEnumerator10" :`NewEnumerator3` "NewEnumerator4" :!type "/Game/Core/Building/Enum/E_Dock_StaticMeshInfo Enum"))))))
    (else
      (bind _keys_2 (`BlueprintMapLibrary.Map_Keys` InPipelineContactInfo))
      (bind _output_2 (`|GetArrayItem` _keys_2))
      (bind _pipelineorbuilding (break `/Game/Core/Building/Struct/TransportNetwork/ST_PipelineContactInfo` (`BlueprintMapLibrary.Map_Find` InPipelineContactInfo _output_2)))
      (if _pipelineorbuilding
        (set `local.TempPipeEnum` _output_2)
        (else
          (set `local.TempBuildingEnum` _output_2)))
      (bind _output_3 (`|GetArrayItem` _keys_2 1))
      (bind _pipelineorbuilding_2 (break `/Game/Core/Building/Struct/TransportNetwork/ST_PipelineContactInfo` (`BlueprintMapLibrary.Map_Find` InPipelineContactInfo _output_3)))
      (if _pipelineorbuilding_2
        (set `local.TempPipeEnum` _output_3)
        (else
          (set `local.TempBuildingEnum` _output_3)))
      (if (== _pipelineorbuilding _pipelineorbuilding_2)
        (return "NewEnumerator0")
        (else
          (return (select `/Game/Core/Building/Enum/E_ContactInfo` (`local.TempBuildingEnum`) :`NewEnumerator0` (select `/Game/Core/Building/Enum/E_ContactInfo` (`local.TempPipeEnum`) :`NewEnumerator0` "NewEnumerator0" :`NewEnumerator1` (enumliteral `/Game/Core/Building/Enum/E_Dock_StaticMeshInfo` "NewEnumerator1") :`NewEnumerator2` (enumliteral `/Game/Core/Building/Enum/E_Dock_StaticMeshInfo` "NewEnumerator2") :`NewEnumerator3` (enumliteral `/Game/Core/Building/Enum/E_Dock_StaticMeshInfo` "NewEnumerator3")) :`NewEnumerator1` (select `/Game/Core/Building/Enum/E_ContactInfo` (`local.TempPipeEnum`) :`NewEnumerator0` (enumliteral `/Game/Core/Building/Enum/E_Dock_StaticMeshInfo` "NewEnumerator7") :`NewEnumerator1` "NewEnumerator0" :`NewEnumerator2` (enumliteral `/Game/Core/Building/Enum/E_Dock_StaticMeshInfo` "NewEnumerator9") :`NewEnumerator3` (enumliteral `/Game/Core/Building/Enum/E_Dock_StaticMeshInfo` "NewEnumerator8")) :`NewEnumerator2` (select `/Game/Core/Building/Enum/E_ContactInfo` (`local.TempPipeEnum`) :`NewEnumerator0` (enumliteral `/Game/Core/Building/Enum/E_Dock_StaticMeshInfo` "NewEnumerator12") :`NewEnumerator1` (enumliteral `/Game/Core/Building/Enum/E_Dock_StaticMeshInfo` "NewEnumerator11") :`NewEnumerator2` "NewEnumerator0" :`NewEnumerator3` (enumliteral `/Game/Core/Building/Enum/E_Dock_StaticMeshInfo` "NewEnumerator10")) :`NewEnumerator3` (select `/Game/Core/Building/Enum/E_ContactInfo` (`local.TempPipeEnum`) :`NewEnumerator0` (enumliteral `/Game/Core/Building/Enum/E_Dock_StaticMeshInfo` "NewEnumerator5") :`NewEnumerator1` (enumliteral `/Game/Core/Building/Enum/E_Dock_StaticMeshInfo` "NewEnumerator6") :`NewEnumerator2` (enumliteral `/Game/Core/Building/Enum/E_Dock_StaticMeshInfo` "NewEnumerator4") :`NewEnumerator3` "NewEnumerator0"))))))))

(fn `InteractWithBuilding`)

(fn `OnAfterInitialization`
  (locals (TempInt :type Integer))
  (`parent.OnAfterInitialization`))

(fn `PipelineTickLoop`
  (params (DeltaSeconds :type "Float (double-precision)" :default 0.0))
  (returns (OutResult :type Boolean) (OutSuccessNum :type Integer))
  ;[1 1 1] If dock do not select passing by item
)

(fn `RefreshPSNode`
  (bind _pipelinecontactinfo (`self.PipelineContactInfo`))
  (if (`.bSuccess` (cast `/Game/Core/Building/Blueprint/BP_Building_OutputDock` self :!pure true))
    (bind _values (`BlueprintMapLibrary.Map_Values` _pipelinecontactinfo))
    (for _array_element _values
      (bind (_pipelineorbuilding _contactedpipeline _contactedbuilding) (break `/Game/Core/Building/Struct/TransportNetwork/ST_PipelineContactInfo` _array_element))
      (if _pipelineorbuilding
        (set `self.SuccessorNode` _contactedpipeline)
        (set `/Game/Core/Building/Blueprint/BP_Building_Pipeline.PrecursorNode` self _contactedpipeline)
        (else
          (set `self.ContactBuilding` _contactedbuilding))))
    (else
      (bind _values_2 (`BlueprintMapLibrary.Map_Values` _pipelinecontactinfo))
      (for _array_element_2 _values_2
        (bind (_pipelineorbuilding_2 _contactedpipeline_2 _contactedbuilding_2) (break `/Game/Core/Building/Struct/TransportNetwork/ST_PipelineContactInfo` _array_element_2))
        (if _pipelineorbuilding_2
          (set `self.PrecursorNode` _contactedpipeline_2)
          (set `/Game/Core/Building/Blueprint/BP_Building_Pipeline.SuccessorNode` self _contactedpipeline_2)
          (else
            (set `self.ContactBuilding` _contactedbuilding_2)))))))

(fn `SetCurrentPassingItems`
  (params (`InMisc.` :type "/Game/Core/Item/Enum/E_Miscellaneous Enum" :default "NewEnumerator73"))
  (returns (OutResult :type Boolean)))

(fn `UserConstructionScript`
  (`parent.UserConstructionScript`))