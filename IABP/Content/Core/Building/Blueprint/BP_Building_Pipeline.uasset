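; Pipeline building piece that auto-tiles into straight, corner, T or cross meshes to match adjacent pipes.
; After initialization it line-traces four sides for other pipelines, then picks a mesh index from the contacts, falling back to index 0 on transport network conflicts.
; When networks agree, it inherits a neighbor's network ID and in/out data.
; It then has each neighbor re-trace and update its mesh by shape alone, ignoring networks.
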(fn `ChangeCurrentStaticMesh`
  (bind _rightcontactpipe (`self.RightContactPipe`))
  (bind _upcontactpipe (`self.UpContactPipe`))
  (bind _downcontactpipe (`self.DownContactPipe`))
  (bind _leftcontactpipe (`self.LeftContactPipe`))
  (bind _outstaticmeshindex (`self.Check Content State`))
  (`self.ChangeStaticMesh` _outstaticmeshindex)
  (`|ExecutionSequence`
    (:`then_0`
      (`/Engine/EditorBlueprintResources/StandardMacros.IsValid` _upcontactpipe
        (:`Is Valid`
          (bind _outstaticmeshindex_2 (`self.CheckStaticMeshCorrect` _upcontactpipe))
          (`self.ChangeStaticMesh` _upcontactpipe _outstaticmeshindex_2))))
    (:`then_1`
      (`/Engine/EditorBlueprintResources/StandardMacros.IsValid` _downcontactpipe
        (:`Is Valid`
          (bind _outstaticmeshindex_3 (`self.CheckStaticMeshCorrect` _downcontactpipe))
          (`self.ChangeStaticMesh` _downcontactpipe _outstaticmeshindex_3))))
    (:`then_2`
      (`/Engine/EditorBlueprintResources/StandardMacros.IsValid` _leftcontactpipe
        (:`Is Valid`
          (bind _outstaticmeshindex_4 (`self.CheckStaticMeshCorrect` _leftcontactpipe))
          (`self.ChangeStaticMesh` _leftcontactpipe _outstaticmeshindex_4))))
    (:`then_3`
      (`/Engine/EditorBlueprintResources/StandardMacros.IsValid` _rightcontactpipe
        (:`Is Valid`
          (bind _outstaticmeshindex_5 (`self.CheckStaticMeshCorrect` _rightcontactpipe))
          (`self.ChangeStaticMesh` _rightcontactpipe _outstaticmeshindex_5))))))

(fn `ChangeStaticMesh`
  (params (InChangeStaticMesh :type Integer))
  (if (== InChangeStaticMesh (`KismetStringLibrary.Conv_StringToInt` (`.RightS` (`KismetStringLibrary.Split` (`KismetSystemLibrary.GetObjectName` (`StaticMeshComponent.StaticMesh` (`self.MainBuilding`))) "_" "IgnoreCase" "FromEnd"))))
    (return)
    (else
      (`StaticMeshComponent.SetStaticMesh` (`self.MainBuilding`) (`|GetArrayItem` (`self.StaticMeshSet`) InChangeStaticMesh))
      (return))))

(fn `Check Content State`
  (returns (OutStaticMeshIndex :type Integer))
  (bind _currenttransformnetwork (`/Game/Core/Building/Blueprint/BP_Building_Pipeline.CurrentTransformNetwork` (`self.DownContactPipe`)))
  (bind _currenttransformnetwork_2 (`/Game/Core/Building/Blueprint/BP_Building_Pipeline.CurrentTransformNetwork` (`self.LeftContactPipe`)))
  (bind _currenttransformnetwork_3 (`/Game/Core/Building/Blueprint/BP_Building_Pipeline.CurrentTransformNetwork` (`self.LeftContactPipe`)))
  (bind _currenttransformnetwork_4 (`/Game/Core/Building/Blueprint/BP_Building_Pipeline.CurrentTransformNetwork` (`self.DownContactPipe`)))
  (bind _currenttransformnetwork_5 (`/Game/Core/Building/Blueprint/BP_Building_Pipeline.CurrentTransformNetwork` (`self.DownContactPipe`)))
  (bind _currenttransformnetwork_6 (`/Game/Core/Building/Blueprint/BP_Building_Pipeline.CurrentTransformNetwork` (`self.DownContactPipe`)))
  ;[1 1 1] Check is cross pipeline
  (if (and (`self.ContactLeft`) (`self.ContactRight`) (`self.ContactUp`) (`self.ContactDown`))
    ;[1 1 1] Check the transform network is same, if not keep normal and add material flash
    (if (and (== (`/Game/Core/Building/Blueprint/BP_Building_Pipeline.CurrentTransformNetwork` (`self.UpContactPipe`)) _currenttransformnetwork) (== _currenttransformnetwork _currenttransformnetwork_2) (== _currenttransformnetwork_2 (`/Game/Core/Building/Blueprint/BP_Building_Pipeline.CurrentTransformNetwork` (`self.RightContactPipe`))))
      (`self.UsingParentInfos` (`self.UpContactPipe`))
      (return 11)
      (else
        (return 0)))
    (else
      ;[1 1 1] Check is T pipeline
      (if (and (`self.ContactLeft`) (`self.ContactRight`) (`self.ContactUp`))
        (if (and (== (`/Game/Core/Building/Blueprint/BP_Building_Pipeline.CurrentTransformNetwork` (`self.UpContactPipe`)) _currenttransformnetwork_3) (== _currenttransformnetwork_3 (`/Game/Core/Building/Blueprint/BP_Building_Pipeline.CurrentTransformNetwork` (`self.RightContactPipe`))))
          (`self.UsingParentInfos` (`self.UpContactPipe`))
          (return 7)
          (else
            (return 0)))
        (elif (and (`self.ContactDown`) (`self.ContactRight`) (`self.ContactUp`))
          (if (and (== (`/Game/Core/Building/Blueprint/BP_Building_Pipeline.CurrentTransformNetwork` (`self.UpContactPipe`)) _currenttransformnetwork_4) (== _currenttransformnetwork_4 (`/Game/Core/Building/Blueprint/BP_Building_Pipeline.CurrentTransformNetwork` (`self.RightContactPipe`))))
            (`self.UsingParentInfos` (`self.UpContactPipe`))
            (return 8)
            (else
              (return 0)))
          (elif (and (`self.ContactDown`) (`self.ContactRight`) (`self.ContactLeft`))
            (if (and (== (`/Game/Core/Building/Blueprint/BP_Building_Pipeline.CurrentTransformNetwork` (`self.LeftContactPipe`)) _currenttransformnetwork_5) (== _currenttransformnetwork_5 (`/Game/Core/Building/Blueprint/BP_Building_Pipeline.CurrentTransformNetwork` (`self.RightContactPipe`))))
              (`self.UsingParentInfos` (`self.DownContactPipe`))
              (return 9)
              (else
                (return 0)))
            (elif (and (`self.ContactDown`) (`self.ContactUp`) (`self.ContactLeft`))
              (if (and (== (`/Game/Core/Building/Blueprint/BP_Building_Pipeline.CurrentTransformNetwork` (`self.LeftContactPipe`)) _currenttransformnetwork_6) (== _currenttransformnetwork_6 (`/Game/Core/Building/Blueprint/BP_Building_Pipeline.CurrentTransformNetwork` (`self.UpContactPipe`))))
                (`self.UsingParentInfos` (`self.UpContactPipe`))
                (return 10)
                (else
                  (return 0)))
              (else
                ;[1 1 1] Check is L pipeline
                (if (and (`self.ContactDown`) (`self.ContactRight`))
                  (if (== (`/Game/Core/Building/Blueprint/BP_Building_Pipeline.CurrentTransformNetwork` (`self.RightContactPipe`)) (`/Game/Core/Building/Blueprint/BP_Building_Pipeline.CurrentTransformNetwork` (`self.DownContactPipe`)))
                    (`self.UsingParentInfos` (`self.DownContactPipe`))
                    (return 3)
                    (else
                      (return 0)))
                  (elif (and (`self.ContactUp`) (`self.ContactRight`))
                    (if (== (`/Game/Core/Building/Blueprint/BP_Building_Pipeline.CurrentTransformNetwork` (`self.RightContactPipe`)) (`/Game/Core/Building/Blueprint/BP_Building_Pipeline.CurrentTransformNetwork` (`self.UpContactPipe`)))
                      (`self.UsingParentInfos` (`self.UpContactPipe`))
                      (return 4)
                      (else
                        (return 0)))
                    (elif (and (`self.ContactUp`) (`self.ContactLeft`))
                      (if (== (`/Game/Core/Building/Blueprint/BP_Building_Pipeline.CurrentTransformNetwork` (`self.LeftContactPipe`)) (`/Game/Core/Building/Blueprint/BP_Building_Pipeline.CurrentTransformNetwork` (`self.UpContactPipe`)))
                        (`self.UsingParentInfos` (`self.UpContactPipe`))
                        (return 5)
                        (else
                          (return 0)))
                      (elif (and (`self.ContactLeft`) (`self.ContactDown`))
                        (if (== (`/Game/Core/Building/Blueprint/BP_Building_Pipeline.CurrentTransformNetwork` (`self.LeftContactPipe`)) (`/Game/Core/Building/Blueprint/BP_Building_Pipeline.CurrentTransformNetwork` (`self.DownContactPipe`)))
                          (`self.UsingParentInfos` (`self.DownContactPipe`))
                          (return 6)
                          (else
                            (return 0)))
                        (else
                          ;[1 1 1] Check is I pipeline
                          (if (and (`self.ContactUp`) (`self.ContactDown`))
                            (if (== (`/Game/Core/Building/Blueprint/BP_Building_Pipeline.CurrentTransformNetwork` (`self.UpContactPipe`)) (`/Game/Core/Building/Blueprint/BP_Building_Pipeline.CurrentTransformNetwork` (`self.DownContactPipe`)))
                              (`self.UsingParentInfos` (`self.UpContactPipe`))
                              (return 1)
                              (else
                                (return 0)))
                            (elif (and (`self.ContactLeft`) (`self.ContactRight`))
                              (if (== (`/Game/Core/Building/Blueprint/BP_Building_Pipeline.CurrentTransformNetwork` (`self.LeftContactPipe`)) (`/Game/Core/Building/Blueprint/BP_Building_Pipeline.CurrentTransformNetwork` (`self.RightContactPipe`)))
                                (`self.UsingParentInfos` (`self.RightContactPipe`))
                                (return 2)
                                (else
                                  (return 0)))
                              (elif (`self.ContactUp`)
                                (if (!= (`/Game/Core/Building/Blueprint/BP_Building_Pipeline.CurrentTransformNetwork` (`self.UpContactPipe`)) -1)
                                  (`self.UsingParentInfos` (`self.UpContactPipe`))
                                  (return 1)
                                  (else
                                    (return 0)))
                                (elif (`self.ContactDown`)
                                  (if (!= (`/Game/Core/Building/Blueprint/BP_Building_Pipeline.CurrentTransformNetwork` (`self.DownContactPipe`)) -1)
                                    (`self.UsingParentInfos` (`self.DownContactPipe`))
                                    (return 1)
                                    (else
                                      (return 0)))
                                  (elif (`self.ContactLeft`)
                                    (if (!= (`/Game/Core/Building/Blueprint/BP_Building_Pipeline.CurrentTransformNetwork` (`self.LeftContactPipe`)) -1)
                                      (`self.UsingParentInfos` (`self.LeftContactPipe`))
                                      (return 2)
                                      (else
                                        (return 0)))
                                    (elif (`self.ContactRight`)
                                      (if (!= (`/Game/Core/Building/Blueprint/BP_Building_Pipeline.CurrentTransformNetwork` (`self.RightContactPipe`)) -1)
                                        (`self.UsingParentInfos` (`self.RightContactPipe`))
                                        (return 2)
                                        (else
                                          (return 0)))
                                      (else
                                        (return 1)))))))))))))))))))))

(fn `CheckStaticMeshCorrect`
  (returns (OutStaticMeshIndex :type Integer))
  (bind _returnvalue (`SceneComponent.K2_GetComponentLocation` (`self.MainBuilding`)))
  ;[1 1 1] Check Up
  (bind (_outhit _returnvalue_2) (`KismetSystemLibrary.LineTraceSingle` :`Start` (+ _returnvalue (`self.UpVectorBase`)) :`End` (+ _returnvalue (`self.UpVector`)) :`TraceChannel` "TraceTypeQuery1" :`DrawDebugType` "Persistent"))
  (if _returnvalue_2
    (bind _asbp_building_pipeline (cast `/Game/Core/Building/Blueprint/BP_Building_Pipeline` (`.HitActor` (`GameplayStatics.BreakHitResult` _outhit)))
      (:`then`
        (set `self.ContactUp` true)
        (set `self.UpContactPipe` _asbp_building_pipeline))
      (:`CastFailed`
        _)))
  ;[1 1 1] Check Down
  (bind (_outhit_2 _returnvalue_3) (`KismetSystemLibrary.LineTraceSingle` :`Start` (+ _returnvalue (`self.DownVectorBase`)) :`End` (+ _returnvalue (`self.DownVector`)) :`TraceChannel` "TraceTypeQuery1" :`DrawDebugType` "Persistent"))
  (if _returnvalue_3
    (bind _asbp_building_pipeline_2 (cast `/Game/Core/Building/Blueprint/BP_Building_Pipeline` (`.HitActor` (`GameplayStatics.BreakHitResult` _outhit_2)))
      (:`then`
        (set `self.ContactDown` true)
        (set `self.DownContactPipe` _asbp_building_pipeline_2))
      (:`CastFailed`
        _)))
  ;[1 1 1] Check Left
  (bind (_outhit_3 _returnvalue_4) (`KismetSystemLibrary.LineTraceSingle` :`Start` (+ _returnvalue (`self.LeftVectorBase`)) :`End` (+ _returnvalue (`self.LeftVector`)) :`TraceChannel` "TraceTypeQuery1" :`DrawDebugType` "Persistent"))
  (if _returnvalue_4
    (bind _asbp_building_pipeline_3 (cast `/Game/Core/Building/Blueprint/BP_Building_Pipeline` (`.HitActor` (`GameplayStatics.BreakHitResult` _outhit_3)))
      (:`then`
        (set `self.ContactLeft` true)
        (set `self.LeftContactPipe` _asbp_building_pipeline_3))
      (:`CastFailed`
        _)))
  ;[1 1 1] Check Right
  (bind (_outhit_4 _returnvalue_5) (`KismetSystemLibrary.LineTraceSingle` :`Start` (+ _returnvalue (`self.RightVectorBase`)) :`End` (+ _returnvalue (`self.RightVector`)) :`TraceChannel` "TraceTypeQuery1" :`DrawDebugType` "Persistent"))
  (if _returnvalue_5
    (bind _asbp_building_pipeline_4 (cast `/Game/Core/Building/Blueprint/BP_Building_Pipeline` (`.HitActor` (`GameplayStatics.BreakHitResult` _outhit_4)))
      (:`then`
        (set `self.ContactRight` true)
        (set `self.RightContactPipe` _asbp_building_pipeline_4))
      (:`CastFailed`
        _)))
  ;[1 1 1] Check is cross pipeline
  (if (and (`self.ContactLeft`) (`self.ContactRight`) (`self.ContactUp`) (`self.ContactDown`))
    (return 11)
    (else
      ;[1 1 1] Check is T pipeline
      (if (and (`self.ContactLeft`) (`self.ContactRight`) (`self.ContactUp`))
        (return 7)
        (elif (and (`self.ContactDown`) (`self.ContactRight`) (`self.ContactUp`))
          (return 8)
          (elif (and (`self.ContactDown`) (`self.ContactRight`) (`self.ContactLeft`))
            (return 9)
            (elif (and (`self.ContactDown`) (`self.ContactUp`) (`self.ContactLeft`))
              (return 10)
              (else
                ;[1 1 1] Check is L pipeline
                (if (and (`self.ContactDown`) (`self.ContactRight`))
                  (return 3)
                  (elif (and (`self.ContactUp`) (`self.ContactRight`))
                    (return 4)
                    (elif (and (`self.ContactUp`) (`self.ContactLeft`))
                      (return 5)
                      (elif (and (`self.ContactLeft`) (`self.ContactDown`))
                        (return 6)
                        (else
                          ;[1 1 1] Check is I pipeline
                          (if (and (`self.ContactUp`) (`self.ContactDown`))
                            (return 1)
                            (elif (and (`self.ContactLeft`) (`self.ContactRight`))
                              (return 2)
                              (elif (`self.ContactUp`)
                                (return 1)
                                (elif (`self.ContactDown`)
                                  (return 1)
                                  (elif (`self.ContactLeft`)
                                    (return 2)
                                    (elif (`self.ContactRight`)
                                      (return 2)
                                      (else
                                        (return 1)))))))))))))))))))))

(fn `OnAfterInitialization`
  (bind _returnvalue (`SceneComponent.K2_GetComponentLocation` (`self.MainBuilding`)))
  (`parent.OnAfterInitialization`)
  ;[1 1 1] Check Up
  (bind (_outhit _returnvalue_2) (`KismetSystemLibrary.LineTraceSingle` :`Start` (+ _returnvalue (`self.UpVectorBase`)) :`End` (+ _returnvalue (`self.UpVector`)) :`TraceChannel` "TraceTypeQuery1" :`DrawDebugType` "Persistent"))
  (if _returnvalue_2
    (bind _asbp_building_pipeline (cast `/Game/Core/Building/Blueprint/BP_Building_Pipeline` (`.HitActor` (`GameplayStatics.BreakHitResult` _outhit)))
      (:`then`
        (set `self.ContactUp` true)
        (set `self.UpContactPipe` _asbp_building_pipeline))
      (:`CastFailed`
        _)))
  ;[1 1 1] Check Down
  (bind (_outhit_2 _returnvalue_3) (`KismetSystemLibrary.LineTraceSingle` :`Start` (+ _returnvalue (`self.DownVectorBase`)) :`End` (+ _returnvalue (`self.DownVector`)) :`TraceChannel` "TraceTypeQuery1" :`DrawDebugType` "Persistent"))
  (if _returnvalue_3
    (bind _asbp_building_pipeline_2 (cast `/Game/Core/Building/Blueprint/BP_Building_Pipeline` (`.HitActor` (`GameplayStatics.BreakHitResult` _outhit_2)))
      (:`then`
        (set `self.ContactDown` true)
        (set `self.DownContactPipe` _asbp_building_pipeline_2))
      (:`CastFailed`
        _)))
  ;[1 1 1] Check Left
  (bind (_outhit_3 _returnvalue_4) (`KismetSystemLibrary.LineTraceSingle` :`Start` (+ _returnvalue (`self.LeftVectorBase`)) :`End` (+ _returnvalue (`self.LeftVector`)) :`TraceChannel` "TraceTypeQuery1" :`DrawDebugType` "Persistent"))
  (if _returnvalue_4
    (bind _asbp_building_pipeline_3 (cast `/Game/Core/Building/Blueprint/BP_Building_Pipeline` (`.HitActor` (`GameplayStatics.BreakHitResult` _outhit_3)))
      (:`then`
        (set `self.ContactLeft` true)
        (set `self.LeftContactPipe` _asbp_building_pipeline_3))
      (:`CastFailed`
        _)))
  ;[1 1 1] Check Right
  (bind (_outhit_4 _returnvalue_5) (`KismetSystemLibrary.LineTraceSingle` :`Start` (+ _returnvalue (`self.RightVectorBase`)) :`End` (+ _returnvalue (`self.RightVectorBase`)) :`TraceChannel` "TraceTypeQuery1" :`DrawDebugType` "Persistent"))
  (if _returnvalue_5
    (bind _asbp_building_pipeline_4 (cast `/Game/Core/Building/Blueprint/BP_Building_Pipeline` (`.HitActor` (`GameplayStatics.BreakHitResult` _outhit_4)))
      (:`then`
        (set `self.ContactRight` true)
        (set `self.RightContactPipe` _asbp_building_pipeline_4))
      (:`CastFailed`
        _)))
  ;[1 1 1] Change Current Static Mesh
  (`self.ChangeCurrentStaticMesh`))

(fn `ProductEffectiveRemoved`
  (params (InIntParam :type Integer) (InTerms :type "Array of /Game/Core/Term/Struct/ST_Term Structure (by ref)"))
  (`parent.ProductEffectiveRemoved` InIntParam InTerms)
  (return))

(fn `RegisterTheTransformNetwork`
  (if (!= (`self.CurrentTransformNetwork`) -1)
    (bind _asbp_global_monitor (cast `/Game/Core/GlobalMonitor/Blueprint/BP_GlobalMonitor` (`GameplayStatics.GetGameState`)))
    (`/Game/Core/GlobalMonitor/Blueprint/BP_GlobalMonitor.TryRegistIntoTransportNetwork` _asbp_global_monitor (`self.CurrentTransformNetwork`))
    (else
      (`/Game/Core/GlobalMonitor/Blueprint/BP_GlobalMonitor.RegistNewTransportNetwork` _asbp_global_monitor))))

(fn `UserConstructionScript`
  (`parent.UserConstructionScript`))

(fn `UsingParentInfos`
  (params (InParentInfos :type "/Game/Core/Building/Blueprint/BP_Building_Pipeline Object Reference"))
  (bind _currenttransformnetwork (`/Game/Core/Building/Blueprint/BP_Building_Pipeline.CurrentTransformNetwork` InParentInfos))
  (bind _currentoutbp (`/Game/Core/Building/Blueprint/BP_Building_Pipeline.CurrentOutBP` InParentInfos))
  (bind _currentinbp (`/Game/Core/Building/Blueprint/BP_Building_Pipeline.CurrentInBP` InParentInfos))
  (`/Engine/EditorBlueprintResources/StandardMacros.IsValid` InParentInfos
    (:`Is Valid`
      (if (!= _currenttransformnetwork -1)
        (set `self.CurrentTransformNetwork` _currenttransformnetwork))
      (if (not (`KismetArrayLibrary.Array_IsEmpty` _currentoutbp))
        (set `self.CurrentOutBP` _currentoutbp))
      (if (not (`KismetArrayLibrary.Array_IsEmpty` _currentinbp))
        (set `self.CurrentInBP` _currentinbp))
      (return))
    (:`Is Not Valid`
      (return))))