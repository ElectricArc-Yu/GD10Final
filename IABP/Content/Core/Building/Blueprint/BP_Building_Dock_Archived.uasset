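; Archived dock building that links a pipeline to a building, with input and output dock variants checked by casting self.
; On mesh refresh it line-traces each contact direction, records pipeline or building hits, and picks an orientation mesh from them.
; After initialization it takes passable items from the building's recipe and adds the first contact's pipeline as successor.
; Input docks accept only the current passing item; the output-pull tick logic is unreachable.
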(event `self.ReceiveTick`
  (params (DeltaSeconds :type "Float (single-precision)"))
  (`parent.ReceiveTick` DeltaSeconds))

(event `self.Event Refresh Static Mesh`
  (`BlueprintMapLibrary.Map_Clear` (`self.PipelineContactInfo`))
  (bind _enumvalue (foreach `/Game/Core/Building/Enum/E_ContactInfo` true)
    (:`LoopBody`
      (`self.CastRayToCheckContact` _enumvalue))
    (:`then`
      (bind _outdockstaticmeshinfo (`self.GetCorrectDockStaticMeshInfo` (`self.PipelineContactInfo`)))
      (`self.ChangeStaticMeshByEnum` "NewEnumerator11" _outdockstaticmeshinfo)
      (`self.InitThePreSuccNode`))))

(fn `CastRayToCheckContact`
  (params (InDerection :type "/Game/Core/Building/Enum/E_ContactInfo Enum" :default "NewEnumerator0"))
  (locals (TempOrigin :type "Vector Structure") (TempDerection :type "Vector Structure"))
  (bind _returnvalue (`SceneComponent.K2_GetComponentLocation` (`self.MainBuilding`)))
  (bind (_origin _derection) (break `/Game/Core/Building/Struct/TransportNetwork/ST_RayInfo` (`BlueprintMapLibrary.Map_Find` (`self.RaycastMap`) InDerection)))
  (set `local.TempOrigin` _origin)
  (set `local.TempDerection` _derection)
  (bind (_outhit _returnvalue_2) (`KismetSystemLibrary.LineTraceSingle` :`Start` (+ _returnvalue (`local.TempOrigin`)) :`End` (+ _returnvalue (`local.TempDerection`)) :`TraceChannel` "TraceTypeQuery1" :`DrawDebugType` (`self.Draw Debug Type`)))
  (if _returnvalue_2
    (bind (_bblockinghit _binitialoverlap _time _distance _location _impactpoint _normal _impactnormal _physmat _hitactor) (`GameplayStatics.BreakHitResult` _outhit))
    (bind _asbp_building (cast `/Game/Core/Building/Blueprint/BP_Building` _hitactor)
      (:`then`
        (bind _asbp_building_pipeline (cast `/Game/Core/Building/Blueprint/BP_Building_Pipeline_Archived` _hitactor)
          (:`then`
            (`BlueprintMapLibrary.Map_Add` (`self.PipelineContactInfo`) (`local.InDerection`) (make `/Game/Core/Building/Struct/TransportNetwork/ST_PipelineContactInfo` true _asbp_building_pipeline null))
            (return))
          (:`CastFailed`
            (`BlueprintMapLibrary.Map_Add` (`self.PipelineContactInfo`) (`local.InDerection`) (make `/Game/Core/Building/Struct/TransportNetwork/ST_PipelineContactInfo` false null _asbp_building))
            (return))))
      (:`CastFailed`
        (return)))
    (else
      (return))))

(fn `GetCorrectDockStaticMeshInfo`
  (params (InPipelineContactInfo :type "Map of /Game/Core/Building/Enum/E_ContactInfo Enum to /Game/Core/Building/Struct/TransportNetwork/ST_PipelineContactInfo Structure"))
  (returns (OutDockStaticMeshInfo :type "/Game/Core/Building/Enum/E_Dock_StaticMeshInfo Enum"))
  (locals (TempBuildingEnum :type "/Game/Core/Building/Enum/E_ContactInfo Enum") (TempPipeEnum :type "/Game/Core/Building/Enum/E_ContactInfo Enum"))
  (if (!= (`BlueprintMapLibrary.Map_Length` InPipelineContactInfo) 2)
    (if (!= (`BlueprintMapLibrary.Map_Length` InPipelineContactInfo) 1)
      (if (> (`BlueprintMapLibrary.Map_Length` InPipelineContactInfo) 2)
        (return "NewEnumerator0")
        (else
          (return "NewEnumerator0")))
      (else
        (bind _keys (`BlueprintMapLibrary.Map_Keys` InPipelineContactInfo))
        (bind _output (`|GetArrayItem` _keys))
        (if (`.PipelineOrBuilding_9_98AA73B24E067DE2AB1C8F83D686ED4F` (break `/Game/Core/Building/Struct/TransportNetwork/ST_PipelineContactInfo` (`BlueprintMapLibrary.Map_Find` InPipelineContactInfo _output)))
          (return (select `/Game/Core/Building/Enum/E_ContactInfo` _output :`NewEnumerator0` "NewEnumerator7" :`NewEnumerator1` "NewEnumerator1" :`NewEnumerator2` "NewEnumerator4" :`NewEnumerator3` "NewEnumerator10" :!type "/Game/Core/Building/Enum/E_Dock_StaticMeshInfo Enum"))
          (else
            (return (select `/Game/Core/Building/Enum/E_ContactInfo` _output :`NewEnumerator0` "NewEnumerator1" :`NewEnumerator1` "NewEnumerator7" :`NewEnumerator2` "NewEnumerator10" :`NewEnumerator3` "NewEnumerator4" :!type "/Game/Core/Building/Enum/E_Dock_StaticMeshInfo Enum"))))))
    (else
      (bind _keys_2 (`BlueprintMapLibrary.Map_Keys` InPipelineContactInfo))
      (bind _output_2 (`|GetArrayItem` _keys_2))
      (bind _pipelineorbuilding (break `/Game/Core/Building/Struct/TransportNetwork/ST_PipelineContactInfo` (`BlueprintMapLibrary.Map_Find` InPipelineContactInfo _output_2)))
      (if _pipelineorbuilding
        (set `local.TempPipeEnum` _output_2)
        (else
          (set `local.TempBuildingEnum` _output_2)))
      (bind _output_3 (`|GetArrayItem` _keys_2 1))
      (bind _pipelineorbuilding_2 (break `/Game/Core/Building/Struct/TransportNetwork/ST_PipelineContactInfo` (`BlueprintMapLibrary.Map_Find` InPipelineContactInfo _output_3)))
      (if _pipelineorbuilding_2
        (set `local.TempPipeEnum` _output_3)
        (else
          (set `local.TempBuildingEnum` _output_3)))
      (if (== _pipelineorbuilding _pipelineorbuilding_2)
        (return "NewEnumerator0")
        (else
          (return (select `/Game/Core/Building/Enum/E_ContactInfo` (`local.TempBuildingEnum`) :`NewEnumerator0` (select `/Game/Core/Building/Enum/E_ContactInfo` (`local.TempPipeEnum`) :`NewEnumerator0` "NewEnumerator0" :`NewEnumerator1` (enumliteral `/Game/Core/Building/Enum/E_Dock_StaticMeshInfo` "NewEnumerator1") :`NewEnumerator2` (enumliteral `/Game/Core/Building/Enum/E_Dock_StaticMeshInfo` "NewEnumerator2") :`NewEnumerator3` (enumliteral `/Game/Core/Building/Enum/E_Dock_StaticMeshInfo` "NewEnumerator3")) :`NewEnumerator1` (select `/Game/Core/Building/Enum/E_ContactInfo` (`local.TempPipeEnum`) :`NewEnumerator0` (enumliteral `/Game/Core/Building/Enum/E_Dock_StaticMeshInfo` "NewEnumerator7") :`NewEnumerator1` "NewEnumerator0" :`NewEnumerator2` (enumliteral `/Game/Core/Building/Enum/E_Dock_StaticMeshInfo` "NewEnumerator9") :`NewEnumerator3` (enumliteral `/Game/Core/Building/Enum/E_Dock_StaticMeshInfo` "NewEnumerator8")) :`NewEnumerator2` (select `/Game/Core/Building/Enum/E_ContactInfo` (`local.TempPipeEnum`) :`NewEnumerator0` (enumliteral `/Game/Core/Building/Enum/E_Dock_StaticMeshInfo` "NewEnumerator12") :`NewEnumerator1` (enumliteral `/Game/Core/Building/Enum/E_Dock_StaticMeshInfo` "NewEnumerator11") :`NewEnumerator2` "NewEnumerator0" :`NewEnumerator3` (enumliteral `/Game/Core/Building/Enum/E_Dock_StaticMeshInfo` "NewEnumerator10")) :`NewEnumerator3` (select `/Game/Core/Building/Enum/E_ContactInfo` (`local.TempPipeEnum`) :`NewEnumerator0` (enumliteral `/Game/Core/Building/Enum/E_Dock_StaticMeshInfo` "NewEnumerator5") :`NewEnumerator1` (enumliteral `/Game/Core/Building/Enum/E_Dock_StaticMeshInfo` "NewEnumerator6") :`NewEnumerator2` "NewEnumerator0" :`NewEnumerator3` (enumliteral `/Game/Core/Building/Enum/E_Dock_StaticMeshInfo` "NewEnumerator4")))))))))

(fn `OnAfterInitialization`
  (locals (TempInt :type Integer))
  (bind (_recipecode _input _output) (break `/Game/Core/Recipe/Struct/ST_Recipe` (`/Game/Core/Building/Blueprint/BP_Building.CurrentRecipe` (`self.ContactBuilding`))))
  (`parent.OnAfterInitialization`)
  (bind _keys (`BlueprintMapLibrary.Map_Keys` (select `bool` (`.bSuccess` (cast `/Game/Core/Building/Blueprint/BP_Building_OutputDock_Archived` self :!pure true)) :`false` _input :`true` _output)))
  (set `self.DockCanPassItems` _keys)
  (bind _values (`BlueprintMapLibrary.Map_Values` (`self.PipelineContactInfo`)))
  (`KismetArrayLibrary.Array_Add` (`self.SuccessorNode`) (`.ContactedPipeline_4_A9D0F1A94D622C3E1286D48D39B8974A` (break `/Game/Core/Building/Struct/TransportNetwork/ST_PipelineContactInfo` (`|GetArrayItem` _values)))))

(fn `PipelineTickLoop`
  (params (DeltaSeconds :type "Float (double-precision)"))
  (returns (OutResult :type Boolean) (OutSuccessNum :type Integer))
  ;[1 1 1] If dock do not select passing by item
)

(fn `ReciveItem`
  (params (InItem :type "/Game/Core/Item/Enum/E_Miscellaneous Enum" :default "NewEnumerator73") (InDeliver :type "/Game/Core/Building/Blueprint/BP_Building_Pipeline_Archived Object Reference"))
  (returns (OutResult :type Boolean))
  (if (`.bSuccess` (cast `/Game/Core/Building/Blueprint/BP_Building_InputDock_Archived` self :!pure true))
    (if (`|EnumEquality` (`self.DockNowPassingItems`) InItem)
      _
      (else
        (return false))))
  (bind _outresult (`parent.ReciveItem` InItem InDeliver))
  (return _outresult))

(fn `SetCurrentPassingItems`
  (params (`InMisc.` :type "/Game/Core/Item/Enum/E_Miscellaneous Enum" :default "NewEnumerator73"))
  (returns (OutResult :type Boolean))
  (if (`KismetArrayLibrary.Array_Contains` (`self.DockCanPassItems`) `InMisc.`)
    (bind _output_get (set `self.DockNowPassingItems` (`self.DockNowPassingItems`)))
    (set `self.KeepedItem` _output_get)
    (set `self.AmountOfKeepingItem` 0)
    (return true)
    (else
      (return false))))

(fn `UserConstructionScript`
  (`parent.UserConstructionScript`))