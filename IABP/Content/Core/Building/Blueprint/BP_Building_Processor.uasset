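; Processor building Blueprint that turns recipe input materials into output products over time.
; Product sets the state sign material by runtime state and, when Normal, advances progress until the cap triggers FinishProduct to update product and material counts.
; Tick rebuilds a debug text readout of stock, progress and power usage; the level line is appended after the string is built, so never displays.
; RemoveProduct is a stub returning false.
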(event `self.ReceiveTick`
  (params (DeltaSeconds :type "Float (single-precision)"))
  (`parent.ReceiveTick` DeltaSeconds)
  (`self.Rerender Debug Log`))

(fn `AfterProduct`
  (params (InDeltaSecond :type "Float (double-precision)"))
  (`parent.AfterProduct` InDeltaSecond))

(fn `FinishProduct`
  (bind _currentproductnum (`self.CurrentProductNum`))
  (bind (_currentrecipe_recipecode _currentrecipe_input _currentrecipe_output) (break `/Game/Core/Recipe/Struct/ST_Recipe` (`self.CurrentRecipe`)))
  (bind _currentmaterialnum (`self.CurrentMaterialNum`))
  (bind _keys (`BlueprintMapLibrary.Map_Keys` _currentrecipe_output))
  (for _array_element _keys
    (bind (_value _returnvalue) (`BlueprintMapLibrary.Map_Find` _currentproductnum _array_element))
    (if (not _returnvalue)
      (`BlueprintMapLibrary.Map_Add` _currentproductnum _array_element))
    (`BlueprintMapLibrary.Map_Add` _currentproductnum _array_element (+ _value (`BlueprintMapLibrary.Map_Find` _currentrecipe_output _array_element))))
  (bind _keys_2 (`BlueprintMapLibrary.Map_Keys` _currentrecipe_input))
  (for _array_element_2 _keys_2
    (`BlueprintMapLibrary.Map_Add` _currentmaterialnum _array_element_2 (- (`BlueprintMapLibrary.Map_Find` _currentmaterialnum _array_element_2) (`BlueprintMapLibrary.Map_Find` _currentrecipe_input _array_element_2))))
  (return))

(fn `Product`
  (params (InRuntimeCode :type "/Game/Core/Building/Enum/E_BuildingRuntimeState Enum" :default "NewEnumerator4") (InDeltaSecond :type "Float (double-precision)"))
  (bind _statesign (`self.StateSign`))
  (bind _returnvalue (+ (* InDeltaSecond (`self.CurrentProgressPerSecond`)) (`self.CurrentProgress`)))
  (`parent.Product` InRuntimeCode InDeltaSecond)
  (bind _output_get (set `self.CurrentState` InRuntimeCode))
  (switch `/Game/Core/Building/Enum/E_BuildingRuntimeState` _output_get
    (:`NewEnumerator4`
      (`PrimitiveComponent.SetMaterial` _statesign 0 "/Game/Arts/StaticMesh/SM_Coal_PowerStation/Material/_lambert6._lambert6"))
    (:`NewEnumerator0`
      (`PrimitiveComponent.SetMaterial` _statesign 0 "/Game/Arts/StaticMesh/SM_Coal_PowerStation/Material/_lambert5._lambert5")
      (if (>= _returnvalue (`self.MaxProgress`))
        ;[1 1 1] Ture then set current progress to 0, and do product incress
        (set `self.CurrentProgress` 0.0)
        (`self.FinishProduct`)
        (else
          (set `self.CurrentProgress` _returnvalue)
          (return))))))

(fn `RemoveProduct`
  (params (InItem :type "/Game/Core/Item/Enum/E_Miscellaneous Enum" :default "NewEnumerator73") (InAmount :type Integer))
  (returns (OutResult :type Boolean))
  (return false))

(fn `Rerender Debug Log`
  (locals (TempText :type "Array of Text") (TempString :type String))
  (bind _maxmaterialnum (`self.MaxMaterialNum`))
  (bind _temptext (`local.TempText`))
  (bind _maxproductnum (`self.MaxProductNum`))
  (bind _temptext_2 (`local.TempText`))
  (set `local.TempString` "")
  (`KismetArrayLibrary.Array_Clear` _temptext)
  (`KismetArrayLibrary.Array_Add` _temptext (`KismetTextLibrary.Conv_StringToText` (`KismetStringLibrary.Concat_StrStr` "" "Material : ")))
  (bind _keys (`BlueprintMapLibrary.Map_Keys` _maxmaterialnum))
  (for _array_element _keys
    (`KismetArrayLibrary.Array_Add` (`local.TempText`) (`KismetTextLibrary.Conv_StringToText` (`KismetStringLibrary.Concat_StrStr` (`|GetEnumeratorNameAsString` _array_element) "  " (`KismetStringLibrary.Conv_IntToString` (`BlueprintMapLibrary.Map_Find` (`self.CurrentMaterialNum`) _array_element)) " / " (`KismetStringLibrary.Conv_IntToString` (`BlueprintMapLibrary.Map_Find` _maxmaterialnum _array_element))))))
  (`KismetArrayLibrary.Array_Add` _temptext (`KismetTextLibrary.Conv_StringToText` (`KismetStringLibrary.Concat_StrStr` "" "Product : ")))
  (bind _keys_2 (`BlueprintMapLibrary.Map_Keys` _maxproductnum))
  (for _array_element_2 _keys_2
    (`KismetArrayLibrary.Array_Add` (`local.TempText`) (`KismetTextLibrary.Conv_StringToText` (`KismetStringLibrary.Concat_StrStr` (`|GetEnumeratorNameAsString` _array_element_2) "  " (`KismetStringLibrary.Conv_IntToString` (`BlueprintMapLibrary.Map_Find` (`self.CurrentProductNum`) _array_element_2)) " / " (`KismetStringLibrary.Conv_IntToString` (`BlueprintMapLibrary.Map_Find` _maxproductnum _array_element_2))))))
  (`KismetArrayLibrary.Array_Add` _temptext_2 (`KismetTextLibrary.Conv_StringToText` (`KismetStringLibrary.Concat_StrStr` "Current progress :  " (`KismetStringLibrary.Conv_DoubleToString` (`self.CurrentProgress`)) " / " (`KismetStringLibrary.Conv_IntToString` (`self.MaxProgress`)) "(" (`KismetStringLibrary.Conv_IntToString` (`self.CurrentProgressPerSecond`)) " / s)")))
  (`KismetArrayLibrary.Array_Add` _temptext_2 (`KismetTextLibrary.Conv_StringToText` (`KismetStringLibrary.Concat_StrStr` "Total Power Usage : " (`KismetTextLibrary.Conv_TextToString` (`KismetTextLibrary.Conv_IntToText` (`self.CurrentTotalEnergyUsage`))))))
  (for _array_element_3 _temptext_2
    (set `local.TempString` (`KismetStringLibrary.Concat_StrStr` (`local.TempString`) (`KismetTextLibrary.Conv_TextToString` _array_element_3) " \n")))
  (`KismetArrayLibrary.Array_Add` _temptext_2 (`KismetTextLibrary.Conv_StringToText` (`KismetStringLibrary.Concat_StrStr` "Current Level : " (`KismetStringLibrary.Conv_IntToString` (`self.CurrentLevel`)) " / " (`KismetStringLibrary.Conv_IntToString` (`self.MaxLevel`)))))
  (`TextRenderComponent.K2_SetText` (`self.Current Recipe`) (`KismetTextLibrary.Conv_StringToText` (`local.TempString`))))

(fn `UserConstructionScript`
  (`parent.UserConstructionScript`))