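; BP_Building_Deliver_01 is a delivery building Blueprint that sells items for money.
; SellingItem looks up the item's price in the PriceList map, multiplies it by the amount, and adds the result to Money on the BP_GlobalMonitor game state.
; ChangePrice is an empty stub, the event graph holds only inactive default events, and the construction script just calls its parent.
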(fn `ChangePrice`)

(fn `SellingItem`
  (params (InItem :type "/Game/Core/Item/Enum/E_Miscellaneous Enum" :default "NewEnumerator73") (InAmount :type Integer))
  (bind _asbp_global_monitor (cast `/Game/Core/GlobalMonitor/Blueprint/BP_GlobalMonitor` (`GameplayStatics.GetGameState`) :!pure true))
  (set `/Game/Core/GlobalMonitor/Blueprint/BP_GlobalMonitor.Money` (+ (* (`BlueprintMapLibrary.Map_Find` (`self.PriceList`) InItem) InAmount) (`/Game/Core/GlobalMonitor/Blueprint/BP_GlobalMonitor.Money` _asbp_global_monitor)) _asbp_global_monitor))

(fn `UserConstructionScript`
  (`parent.UserConstructionScript`))