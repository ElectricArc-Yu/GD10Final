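; Base warehouse building Blueprint that stores and dispenses materials through a capped, index-keyed inventory map.
; TryStorageItem merges into a matching stack within the DT_Miscellaneous MaxStack, otherwise appends a slot if room remains.
; Successful storage calls CheckRecipe, which sets CurrentRecipe to a "None" recipe listing stored materials at zero amount.
; TrySendItem deducts from one sufficient stack, calling MoveAbove on emptied slots, intended to shift later entries down.
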(fn `CheckRecipe`
  (locals (Misc :type "Map of /Game/Core/Item/Enum/E_Miscellaneous Enum to Object Object Reference"))
  (bind _values (`BlueprintMapLibrary.Map_Values` (`self.InventoryItem`)))
  (for _array_element _values
    (`BlueprintMapLibrary.Map_Add` (`local.Misc`) (`.Material_2_37E392C640E74D072EEC269DDA0FEA71` (break `/Game/Core/Building/Struct/Building/ST_BuildingCost` _array_element))))
  (set `self.CurrentRecipe` (make `/Game/Core/Recipe/Struct/ST_Recipe` "None" _ (`local.Misc`))))

(fn `MoveAbove`
  (params (InIndex :type Integer))
  (bind _inventoryitem (`self.InventoryItem`))
  (for _index (range InIndex 1)
    (bind (_value _returnvalue) (`BlueprintMapLibrary.Map_Find` _inventoryitem (+ _index 1)))
    (if _returnvalue
      (`BlueprintMapLibrary.Map_Add` _inventoryitem _index _value)
      (else
        (break))))
  (return))

(fn `TrySendItem`
  (params (InItem :type "/Game/Core/Item/Enum/E_Miscellaneous Enum" :default "NewEnumerator73") (InNum :type Integer))
  (returns (Result :type Boolean))
  (bind _inventoryitem (`self.InventoryItem`))
  (bind _values (`BlueprintMapLibrary.Map_Values` _inventoryitem))
  (for (_array_element _array_index) _values
    (bind (_material _amount) (break `/Game/Core/Building/Struct/Building/ST_BuildingCost` _array_element))
    (if (`|EnumEquality` _material InItem)
      (if (<= InNum _amount)
        (bind _returnvalue (- _amount InNum))
        (if (== _returnvalue 0)
          (`self.MoveAbove` _array_index)
          (return true)
          (else
            (`BlueprintMapLibrary.Map_Add` _inventoryitem _array_index (make `/Game/Core/Building/Struct/Building/ST_BuildingCost` _material _returnvalue))
            (return true))))))
  (return false))

(fn `TryStorageItem`
  (params (InItem :type "/Game/Core/Item/Enum/E_Miscellaneous Enum" :default "NewEnumerator73") (InNum :type Integer))
  (returns (OutResult :type Boolean))
  (locals (IsAdded :type Boolean))
  (bind _inventoryitem (`self.InventoryItem`))
  (bind _inventoryitem_2 (`self.InventoryItem`))
  (bind _returnvalue (`BlueprintMapLibrary.Map_Length` _inventoryitem_2))
  (for _index (range (`self.InventoryMax`))
    (bind (_value _returnvalue_2) (`BlueprintMapLibrary.Map_Find` _inventoryitem _index))
    (if _returnvalue_2
      (bind (_material _amount) (break `/Game/Core/Building/Struct/Building/ST_BuildingCost` _value))
      (if (`|EnumEquality` _material InItem)
        (bind _returnvalue_3 (`|GetDataTableRow` "/Game/Core/Item/Data/DT_Miscellaneous.DT_Miscellaneous" (`|GetEnumeratorName` _material))
          (:`then`
            (bind _returnvalue_4 (+ InNum _amount))
            (if (<= _returnvalue_4 (`.MaxStack_7_94C5F0864067CCDFDA2035861D929B7C` (break `/Game/Core/Item/Struct/ST_Miscellaneous` _returnvalue_3)))
              (`BlueprintMapLibrary.Map_Add` _inventoryitem _index (make `/Game/Core/Building/Struct/Building/ST_BuildingCost` _material _returnvalue_4))
              (set `local.IsAdded` true)
              (break)))))
      (else
        (break))))
  (if (`local.IsAdded`)
    (`self.CheckRecipe`)
    (return true)
    (elif (< _returnvalue (`self.InventoryMax`))
      (`BlueprintMapLibrary.Map_Add` _inventoryitem_2 _returnvalue (make `/Game/Core/Building/Struct/Building/ST_BuildingCost` InItem InNum))
      (`self.CheckRecipe`)
      (return true)
      (else
        (return false)))))

(fn `UserConstructionScript`
  (`parent.UserConstructionScript`))