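; Power generator building Blueprint that adds its power to a shared global power pool while it exists.
; On BeginPlay it looks up its output in the MaxProductNum map by an enum key and registers it with the BP_GlobalMonitor game state.
; Its OnDestory override unregisters the same amount before calling the parent logic.
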(event `self.ReceiveBeginPlay`
  (`parent.ReceiveBeginPlay`)
  (bind _output_get (set `self.PowerAmount` (`BlueprintMapLibrary.Map_Find` (`self.MaxProductNum`) "NewEnumerator74")))
  (`/Game/Core/GlobalMonitor/Blueprint/BP_GlobalMonitor.RegistPower` (cast `/Game/Core/GlobalMonitor/Blueprint/BP_GlobalMonitor` (`GameplayStatics.GetGameState`) :!pure true) _output_get))

(fn `OnDestory`
  (`/Game/Core/GlobalMonitor/Blueprint/BP_GlobalMonitor.UnregistPower` (cast `/Game/Core/GlobalMonitor/Blueprint/BP_GlobalMonitor` (`GameplayStatics.GetGameState`) :!pure true) (`self.PowerAmount`))
  (`parent.OnDestory`))

(fn `UserConstructionScript`
  (`parent.UserConstructionScript`))