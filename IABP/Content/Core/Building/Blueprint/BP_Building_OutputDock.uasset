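; BP_Building_OutputDock is a building that pulls finished products out of its contact building and passes them on for delivery.
; Each Tick, while empty, it selects the contact building's first product type and deducts one batch, sized by TransportingMagnification, once stock suffices.
; While holding an item, it retries TryDeliverItem every Tick until delivery succeeds.
; Only the first MaxProductNum key is ever exported.
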(event `self.ReceiveTick`
  (params (DeltaSeconds :type "Float (single-precision)"))
  (bind _contactbuilding (`self.ContactBuilding`))
  (bind _currentproductnum (`/Game/Core/Building/Blueprint/BP_Building.CurrentProductNum` _contactbuilding))
  (`parent.ReceiveTick` 0.0)
  (if (`self.NowKeepingItem`)
    (bind _outresult (`self.TryDeliverItem`))
    (set `self.NowKeepingItem` (not _outresult))
    (else
      (`/Engine/EditorBlueprintResources/StandardMacros.IsValid` _contactbuilding
        (:`Is Valid`
          (bind _keys (`BlueprintMapLibrary.Map_Keys` (`/Game/Core/Building/Blueprint/BP_Building.MaxProductNum` _contactbuilding)))
          (bind _output_get (set `self.PassingItem` (`|GetArrayItem` _keys)))
          (bind _value (`BlueprintMapLibrary.Map_Find` _currentproductnum _output_get))
          (bind _value_2 (`BlueprintMapLibrary.Map_Find` (`self.TransportingMagnification`) _output_get))
          (if (>= _value _value_2)
            (`BlueprintMapLibrary.Map_Add` _currentproductnum _output_get (- _value _value_2))
            (set `self.NowKeepingItem` true)))))))

(fn `UserConstructionScript`
  (`parent.UserConstructionScript`))