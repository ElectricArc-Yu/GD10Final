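; Global warehouse building that deposits delivered items into the shared global inventory.
; DeliverItemToGlobalInventory casts the Game State to BP_GlobalMonitor and adds the amount to that item's entry in CurrentGlobalInventory, creating the entry if absent.
; The warehouse stores nothing itself and has no active event logic.
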(fn `DeliverItemToGlobalInventory`
  (params (InMisc :type "/Game/Core/Item/Enum/E_Miscellaneous Enum" :default "NewEnumerator73") (InAmount :type Integer))
  (bind _asbp_global_monitor (cast `/Game/Core/GlobalMonitor/Blueprint/BP_GlobalMonitor` (`GameplayStatics.GetGameState`)))
  (bind _currentglobalinventory (`/Game/Core/GlobalMonitor/Blueprint/BP_GlobalMonitor.CurrentGlobalInventory` _asbp_global_monitor))
  (bind (_value _returnvalue) (`BlueprintMapLibrary.Map_Find` _currentglobalinventory (`local.InMisc`)))
  (if _returnvalue
    (`BlueprintMapLibrary.Map_Add` _currentglobalinventory (`local.InMisc`) (+ (`local.InAmount`) _value))
    (else
      (`BlueprintMapLibrary.Map_Add` _currentglobalinventory (`local.InMisc`) (`local.InAmount`)))))

(fn `UserConstructionScript`
  (`parent.UserConstructionScript`))