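; BP_Building_InputDock is a building dock that takes one item at a time from a deliverer and hands it to a connected building.
; ReciveItem rejects items while occupied, otherwise stores the item and finds the contacted building from PipelineContactInfo.
; Tick deposits the amount from TransportingMagnification into a global warehouse, sells it through a Deliver_01 building, or adds it to other buildings' materials.
; Items exceeding material capacity or lacking a slot stay held.
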(event `self.ReceiveTick`
  (params (DeltaSeconds :type "Float (single-precision)"))
  (bind _contactbuilding (`self.ContactBuilding`))
  (bind _passingitem (`self.PassingItem`))
  (bind _value (`BlueprintMapLibrary.Map_Find` (`self.TransportingMagnification`) (`self.PassingItem`)))
  (bind (_asbp_building_global_warehouse _bsuccess) (cast `/Game/Core/Building/Blueprint/BP_Building_GlobalWarehouse` _contactbuilding :!pure true))
  (bind (_asbp_building_deliver_01 _bsuccess_2) (cast `/Game/Core/Building/Blueprint/BP_Building_Deliver_01` _contactbuilding :!pure true))
  (bind _currentmaterialnum (`/Game/Core/Building/Blueprint/BP_Building.CurrentMaterialNum` _contactbuilding))
  (bind (_value_2 _returnvalue) (`BlueprintMapLibrary.Map_Find` _currentmaterialnum _passingitem))
  (bind _returnvalue_2 (+ _value_2 (`BlueprintMapLibrary.Map_Find` (`self.TransportingMagnification`) (`self.PassingItem`))))
  (`parent.ReceiveTick` DeltaSeconds)
  (if (`self.NowKeepingItem`)
    (`/Engine/EditorBlueprintResources/StandardMacros.IsValid` _contactbuilding
      (:`Is Valid`
        (if _bsuccess
          (`/Game/Core/Building/Blueprint/BP_Building_GlobalWarehouse.DeliverItemToGlobalInventory` _asbp_building_global_warehouse (`self.PassingItem`) _value)
          (set `self.NowKeepingItem` false :!label _label)
          (elif _bsuccess_2
            (`/Game/Core/Building/Blueprint/BP_Building_Deliver_01.SellingItem` _asbp_building_deliver_01 (`self.PassingItem`) _value)
            (goto _label)
            (elif _returnvalue
              (if (<= _returnvalue_2 (`BlueprintMapLibrary.Map_Find` (`/Game/Core/Building/Blueprint/BP_Building.MaxMaterialNum` _contactbuilding) (`self.PassingItem`)))
                (`BlueprintMapLibrary.Map_Add` _currentmaterialnum _passingitem _returnvalue_2)
                (goto _label)))))))))

(fn `ReciveItem`
  (params (InItem :type "/Game/Core/Item/Enum/E_Miscellaneous Enum" :default "NewEnumerator73") (InDeliver :type "/Game/Core/Building/Blueprint/BP_Building_Pipeline Object Reference"))
  (returns (OutResult :type Boolean))
  (if (`self.NowKeepingItem`)
    (return false)
    (else
      (set `self.PrecursorNode` InDeliver)
      (bind _values (`BlueprintMapLibrary.Map_Values` (`self.PipelineContactInfo`)))
      (for _array_element _values
        (bind (_pipelineorbuilding _contactedpipeline _contactedbuilding) (break `/Game/Core/Building/Struct/TransportNetwork/ST_PipelineContactInfo` _array_element))
        (if (not _pipelineorbuilding)
          (set `self.ContactBuilding` _contactedbuilding)))
      (set `self.PassingItem` InItem)
      (set `self.NowKeepingItem` true)
      (return true))))

(fn `UserConstructionScript`
  (`parent.UserConstructionScript`))