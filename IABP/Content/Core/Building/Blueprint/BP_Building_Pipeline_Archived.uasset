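; Archived pipeline building that connects to adjacent pipelines and swaps its mesh to match.
; On initialization it line-traces per direction, turns contacts into a bitmask to pick the mesh, and has neighboring pipelines refresh too.
; Contacts become successor nodes, or precursor nodes for the input dock subclass.
; Item transfer through these nodes is disconnected: receive and deliver are stubs, Tick is empty, and the light-material update never runs.
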(event `self.ReceiveTick`
  (params (DeltaSeconds :type "Float (single-precision)")))

(event `Event Refresh Static Mesh`
  (`BlueprintMapLibrary.Map_Clear` (`self.PipelineContactInfo`))
  (bind _enumvalue (foreach `/Game/Core/Building/Enum/E_ContactInfo` false)
    (:`LoopBody`
      (`self.CastRayToCheckContact` _enumvalue))
    (:`then`
      (bind _outpipelinestaticmeshinfo (`self.Get Correct Pipeline Static Mesh Info` (`self.PipelineContactInfo`)))
      (`self.ChangeStaticMeshByEnum` _outpipelinestaticmeshinfo "NewEnumerator0" true)
      (`self.InitThePreSuccNode`))))

(fn `CastRayToCheckContact`
  (params (InDerection :type "/Game/Core/Building/Enum/E_ContactInfo Enum" :default "NewEnumerator0"))
  (locals (TempOrigin :type "Vector Structure") (TempDerection :type "Vector Structure"))
  (bind _returnvalue (`SceneComponent.K2_GetComponentLocation` (`self.MainBuilding`)))
  (bind (_origin _derection) (break `/Game/Core/Building/Struct/TransportNetwork/ST_RayInfo` (`BlueprintMapLibrary.Map_Find` (`self.RaycastMap`) InDerection)))
  (set `local.TempOrigin` _origin)
  (set `local.TempDerection` _derection)
  (bind (_outhit _returnvalue_2) (`KismetSystemLibrary.LineTraceSingle` (+ _returnvalue (`local.TempOrigin`)) (+ _returnvalue (`local.TempDerection`)) "TraceTypeQuery1" false (`|MakeArray` (cast `/Game/Core/GameMode/BP_Player_UI` (`GameplayStatics.GetPlayerPawn` 0) :!pure true) :!type "Actor Object Reference") (`self.Draw Debug Type`)))
  (if _returnvalue_2
    (bind _asbp_building_pipeline (cast `/Game/Core/Building/Blueprint/BP_Building_Pipeline_Archived` (`.HitActor` (`GameplayStatics.BreakHitResult` _outhit)))
      (:`then`
        (`BlueprintMapLibrary.Map_Add` (`self.PipelineContactInfo`) (`local.InDerection`) (make `/Game/Core/Building/Struct/TransportNetwork/ST_PipelineContactInfo` true _asbp_building_pipeline null))
        (return))
      (:`CastFailed`
        (return)))
    (else
      (return))))

(fn `ChangeStaticMeshByEnum`
  (params (InPipelineStatic :type "/Game/Core/Building/Enum/E_PipeLine_StaticMashInfo Enum" :default "NewEnumerator11") (InDockStatic :type "/Game/Core/Building/Enum/E_Dock_StaticMeshInfo Enum" :default "NewEnumerator0") (DockOrPipeline :type Boolean))
  (if DockOrPipeline
    (if (== (`KismetMathLibrary.Conv_ByteToInt` InPipelineStatic) (`self.CurrentStaticMesh`))
      (return)
      (else
        (`StaticMeshComponent.SetStaticMesh` (`self.MainBuilding`) (`BlueprintMapLibrary.Map_Find` (`self.PipelineStaticMeshInfo`) (`local.InPipelineStatic`)))
        (set `self.CurrentStaticMesh` (`KismetMathLibrary.Conv_ByteToInt` (`local.InPipelineStatic`)))
        (return)))
    (elif (== (`KismetMathLibrary.Conv_ByteToInt` InDockStatic) (`self.CurrentStaticMesh`))
      (return)
      (else
        (`StaticMeshComponent.SetStaticMesh` (`self.MainBuilding`) (`BlueprintMapLibrary.Map_Find` (`self.DockStaticMeshInfo`) (`local.InDockStatic`)))
        (set `self.CurrentStaticMesh` (`KismetMathLibrary.Conv_ByteToInt` (`local.InDockStatic`)))
        (return)))))

(fn `Get Correct Pipeline Static Mesh Info`
  (params (InPipelineContactInfo :type "Map of /Game/Core/Building/Enum/E_ContactInfo Enum to /Game/Core/Building/Struct/TransportNetwork/ST_PipelineContactInfo Structure"))
  (returns (OutPipelineStaticMeshInfo :type "/Game/Core/Building/Enum/E_PipeLine_StaticMashInfo Enum"))
  (locals (TempBitmask :type Integer))
  (bind (_bitmaskinfo_00000001 _bitmaskinfo_00000010 _bitmaskinfo_00000100 _bitmaskinfo_00001000) (break `/Game/Core/Building/Struct/FuckUnreal/ST_FuckUnreal_Bitmask` (`self.BitmaskInfo`)))
  (if (== (`BlueprintMapLibrary.Map_Length` InPipelineContactInfo) 0)
    ;[1 1 1] Error
    (return "NewEnumerator11")
    (else
      (bind _keys (`BlueprintMapLibrary.Map_Keys` (`local.InPipelineContactInfo`)))
      (for _array_element _keys
        (set `local.TempBitmask` (+ (`local.TempBitmask`) (select `/Game/Core/Building/Enum/E_ContactInfo` _array_element :`NewEnumerator0` _bitmaskinfo_00000001 :`NewEnumerator1` _bitmaskinfo_00000010 :`NewEnumerator2` _bitmaskinfo_00000100 :`NewEnumerator3` _bitmaskinfo_00001000))))
      (switch `int` (`local.TempBitmask`)
        (:`1`
          _)
        (:`2`
          _)
        (:`3`
          _)
        (:`4`
          (return "NewEnumerator1"))
        (:`5`
          (return "NewEnumerator5"))
        (:`6`
          (return "NewEnumerator4"))
        (:`7`
          (return "NewEnumerator11"))
        (:`8`
          (return "NewEnumerator1"))
        (:`9`
          (return "NewEnumerator2"))
        (:`10`
          (return "NewEnumerator3"))
        (:`11`
          (return "NewEnumerator11"))
        (:`12`
          (return "NewEnumerator1"))
        (:`13`
          (return "NewEnumerator11"))
        (:`14`
          (return "NewEnumerator11"))
        (:`15`
          (return "NewEnumerator11")))
      (return "NewEnumerator0"))))

(fn `InitThePreSuccNode`
  ;[1 1 1] Init the Pre/Succ node
  (bind _values (`BlueprintMapLibrary.Map_Values` (`self.PipelineContactInfo`)))
  (for _array_element _values
    (bind (_pipelineorbuilding _contactedpipeline _contactedbuilding) (break `/Game/Core/Building/Struct/TransportNetwork/ST_PipelineContactInfo` _array_element))
    (if _pipelineorbuilding
      (`KismetArrayLibrary.Array_Add` (`self.SuccessorNode`) _contactedpipeline)
      (else
        (set `self.ContactBuilding` _contactedbuilding))))
  (if (`.bSuccess` (cast `/Game/Core/Building/Blueprint/BP_Building_InputDock_Archived` self :!pure true))
    (set `self.PrecursorNode` (`self.SuccessorNode`))
    (`KismetArrayLibrary.Array_Clear` (`self.SuccessorNode`))))

(fn `OnAfterInitialization`
  (`parent.OnAfterInitialization`)
  (`self.Event Refresh Static Mesh`)
  (bind _values (`BlueprintMapLibrary.Map_Values` (`self.PipelineContactInfo`)))
  (for _array_element _values
    (bind (_pipelineorbuilding _contactedpipeline) (break `/Game/Core/Building/Struct/TransportNetwork/ST_PipelineContactInfo` _array_element))
    (if _pipelineorbuilding
      (`self.Event Refresh Static Mesh` _contactedpipeline)))
  (return))

(fn `PipelineTickLoop`
  (params (DeltaSeconds :type "Float (double-precision)"))
  (returns (OutResult :type Boolean))
  (locals (TempSuccessAmount :type Integer))
  (`/Engine/EditorBlueprintResources/StandardMacros.IncrementInt` (`self.Timer`)
    (:`  `
      (if (>= (`self.Timer`) (`self.Bandwidth`))
        (set `self.Timer` 0)))))

(fn `ProductEffectiveRemoved`
  (params (InIntParam :type Integer) (InTerms :type "Array of /Game/Core/Term/Struct/ST_Term Structure (by ref)"))
  (`parent.ProductEffectiveRemoved` InIntParam InTerms)
  (return))

(fn `ReciveItem`
  (params (InItem :type "/Game/Core/Item/Enum/E_Miscellaneous Enum" :default "NewEnumerator2") (InDeliver :type "/Game/Core/Building/Blueprint/BP_Building_Pipeline_Archived Object Reference"))
  (returns (OutResult :type Boolean)))

(fn `Rerender Debug Log`
  (locals (Temp :type String))
  (bind _textrender (`self.TextRender`))
  (bind _temp (`local.Temp`))
  (bind (_asbp_building_input_dock _bsuccess) (cast `/Game/Core/Building/Blueprint/BP_Building_InputDock_Archived` self :!pure true))
  (if (== (`self.AmountOfKeepingItem`) 0)
    (`TextRenderComponent.SetTextRenderColor` _textrender (make `Color` 255 0 255 255))
    (else
      (`TextRenderComponent.SetTextRenderColor` _textrender (make `Color` 0 255 255 255))))
  (`|ExecutionSequence`
    (:`then_0`
      (if _bsuccess
        (set `local.Temp` (`KismetStringLibrary.Concat_StrStr` _temp "Dock Can Passing Item:"))
        (for _array_element (`/Game/Core/Building/Blueprint/BP_Building_Dock_Archived.DockCanPassItems` _asbp_building_input_dock)
          (set `local.Temp` (`KismetStringLibrary.Concat_StrStr` _temp (`|GetEnumeratorNameAsString` _array_element) " | ")))
        (else
          (set `local.Temp` (`KismetStringLibrary.Concat_StrStr` "Now Keeping Item : " (`|GetEnumeratorNameAsString` (`self.KeepedItem`)) " \n")))))
    (:`then_1`
      (set `local.Temp` (`KismetStringLibrary.Concat_StrStr` (`local.Temp`) "Amount Of Keeping : " (`KismetStringLibrary.Conv_IntToString` (`self.AmountOfKeepingItem`)))))
    (:`then_2`
      (`TextRenderComponent.K2_SetText` (`self.TextRender`) (`KismetTextLibrary.Conv_StringToText` (`local.Temp`))))))

(fn `SetMaterialProperty`
  (if (> (`self.AmountOfKeepingItem`) 0)
    (`PrimitiveComponent.SetMaterialByName` (`self.MainBuilding`) "M_pipe_light" "/Game/Arts/StaticMesh/SM_Coal_PowerStation/Material/_lambert5._lambert5")
    (else
      (`PrimitiveComponent.SetMaterialByName` (`self.MainBuilding`) "M_pipe_light" "/Game/Arts/StaticMesh/SM_Coal_PowerStation/Material/_lambert6._lambert6"))))

(fn `TryDeliverItem`
  (returns (OutResult :type Boolean) (OutSuccessAmount :type Integer))
  (locals (TempFailedAmount :type Integer) (TempSuccessAmount :type Integer)))

(fn `UserConstructionScript`
  (`parent.UserConstructionScript`))