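; Base Blueprint for production buildings, forwarding lifecycle, recipe-change and term-attached events to functions that are mostly placeholder stubs.
; Each tick runs a SelfCheck, Product, AfterProduct pipeline, passing the check's code into production.
; OnRecipeChange loads a recipe from DT_Recipe, takes input and output stack limits from DT_Miscellaneous, then updates progress and energy usage.
; A missing input item row re-triggers the current recipe and fails.
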(event `self.ReceiveBeginPlay`
  (`self.OnInitialization`))

(event `self.ReceiveTick`
  (params (DeltaSeconds :type "Float (single-precision)"))
  (`self.OnTick`))

(event `self.ReceiveDestroyed`
  (`self.OnDestory`))

(event `Event RecipeChange`
  (params (TargetRecipe :type Integer))
  (`self.OnRecipeChange` TargetRecipe))

(event `Event TermAttached`
  (`self.OnTermAttached`))

(fn `AfterProduct`
  (switch `/Game/Core/Building/Enum/E_BuildingRuntimeState` (`self.CurrentState`)))

(fn `OnDestory`)

(fn `OnInitialization`)

(fn `OnRecipeChange`
  (params (InTargetRecipe :type Integer))
  (returns (IsChanged :type Boolean))
  (locals (BackUp :type "/Game/Core/Recipe/Struct/ST_Recipe Structure"))
  ;[1 1 1] Change the recipe
  (bind _returnvalue (`|GetDataTableRow` "/Game/Core/Recipe/Data/DT_Recipe.DT_Recipe" (`KismetStringLibrary.Conv_StringToName` (`KismetStringLibrary.Conv_IntToString` InTargetRecipe)))
    (:`then`
      (bind (_recipecode _input _output _needprogress _energycost) (break `/Game/Core/Recipe/Struct/ST_Recipe` _returnvalue))
      (bind _output_get (set `self.CurrentRecipe` (make `/Game/Core/Recipe/Struct/ST_Recipe` _recipecode _input _output _needprogress _energycost)))
      (bind _keys (`BlueprintMapLibrary.Map_Keys` (`.Input_19_708FD963446AD4B730CD70B992BCFFB3` (break `/Game/Core/Recipe/Struct/ST_Recipe` _output_get))))
      (`BlueprintMapLibrary.Map_Clear` (`self.MaxMaterialNum`))
      (for _array_element _keys
        (bind _returnvalue_2 (`|GetDataTableRow` "/Game/Core/Item/Data/DT_Miscellaneous.DT_Miscellaneous" (`KismetStringLibrary.Conv_StringToName` (`|GetEnumeratorNameAsString` _array_element)))
          (:`then`
            (`BlueprintMapLibrary.Map_Add` (`self.MaxMaterialNum`) _array_element (`.MaxStack_7_94C5F0864067CCDFDA2035861D929B7C` (break `/Game/Core/Item/Struct/ST_Miscellaneous` _returnvalue_2))))
          (:`RowNotFound`
            (`self.Event RecipeChange` (`self.CurrentRecipeName`))
            (return false))))
      (bind _keys_2 (`BlueprintMapLibrary.Map_Keys` (`.Output_18_68B0D3E74CF6E74E1D60E8A7328F314E` (break `/Game/Core/Recipe/Struct/ST_Recipe` _output_get))))
      (`BlueprintMapLibrary.Map_Clear` (`self.MaxProductNum`))
      (for _array_element_2 _keys_2
        (bind _returnvalue_3 (`|GetDataTableRow` "/Game/Core/Item/Data/DT_Miscellaneous.DT_Miscellaneous" (`KismetStringLibrary.Conv_StringToName` (`|GetEnumeratorNameAsString` _array_element_2)))
          (:`then`
            (`BlueprintMapLibrary.Map_Add` (`self.MaxProductNum`) _array_element_2 (`.MaxStack_7_94C5F0864067CCDFDA2035861D929B7C` (break `/Game/Core/Item/Struct/ST_Miscellaneous` _returnvalue_3))))))
      (set `self.MaxProgress` (`.NeedProgress_22_8B8B214E4F8E7220DC96BFA54CD2EC86` (break `/Game/Core/Recipe/Struct/ST_Recipe` _output_get)))
      (set `self.CurrentRecipeName` InTargetRecipe)
      (set `self.CurrentEnergyUsage` (`.EnergyCost_28_4484B983454B0F32086EB4920C4F3768` (break `/Game/Core/Recipe/Struct/ST_Recipe` _output_get)))
      (set `self.CurrentTotalEnergyUsage` (+ (`.EnergyCost_28_4484B983454B0F32086EB4920C4F3768` (break `/Game/Core/Recipe/Struct/ST_Recipe` _output_get)) (`.EnergyCost_63_AEC4D25D406DB390BED6CE8B606539E0` (break `/Game/Core/Building/Struct/ST_Building` (`self.BuildingBaseInfosFromDataTable`)))))
      (return true))
    (:`RowNotFound`
      (return false))))

(fn `OnTermAttached`)

(fn `OnTick`
  (bind _outruntimecode (`self.SelfCheck`))
  (`self.Product` _outruntimecode)
  (`self.AfterProduct`))

(fn `Product`
  (params (InRuntimeCode :type Integer)))

(fn `SelfCheck`
  (returns (OutRuntimeCode :type Integer))
  (return 0))

(fn `UserConstructionScript`)