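; Refinery building Blueprint, a child class in the game's building system with hooks for placement, recipes, production and destruction.
; It adds no logic of its own: every override only calls its parent, so behavior comes from the parent class.
; OnTermAttached passes a constant 0 to the parent instead of forwarding its terminal number.
; BeginPlay and Tick are disabled stubs.
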(fn `AfterDestory`
  (params (InDestoryType :type "/Game/Core/Building/Enum/E_DestoryType Enum" :default "E_DestoryType_MAX"))
  (`parent.AfterDestory` InDestoryType))

(fn `AfterPlace`
  (`parent.AfterPlace`))

(fn `AfterProduct`
  (params (InDeltaSecond :type "Float (double-precision)"))
  (`parent.AfterProduct` InDeltaSecond))

(fn `OnBeforeRecipeChange`
  (params (InTargetRecipe :type Integer))
  (returns (OutInclude :type Boolean))
  (bind _outinclude (`parent.OnBeforeRecipeChange` InTargetRecipe))
  (return _outinclude))

(fn `OnDestory`
  (`parent.OnDestory`))

(fn `OnInitialization`
  (`parent.OnInitialization`))

(fn `OnRecipeChange`
  (params (InTargetRecipe :type Integer))
  (returns (IsChanged :type Boolean))
  (bind _ischanged (`parent.OnRecipeChange` InTargetRecipe))
  (return _ischanged))

(fn `OnTermAttached`
  (params (InTermNo :type Integer))
  (`parent.OnTermAttached` 0))

(fn `OnTick`
  (params (InDeltaSeconds :type "Float (double-precision)"))
  (`parent.OnTick` InDeltaSeconds))

(fn `Product`
  (params (InRuntimeCode :type "/Game/Core/Building/Enum/E_BuildingRuntimeState Enum" :default "NewEnumerator4") (InDeltaSecond :type "Float (double-precision)"))
  (`parent.Product` InRuntimeCode InDeltaSecond))

(fn `SelfCheck`
  (params (InDeltaSecond :type "Float (double-precision)"))
  (returns (OutRuntimeCode :type "/Game/Core/Building/Enum/E_BuildingRuntimeState Enum"))
  (bind _outruntimecode (`parent.SelfCheck` InDeltaSecond))
  (return _outruntimecode))

(fn `UserConstructionScript`
  (`parent.UserConstructionScript`))